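; Game instance for Rivet that exposes save, load, create, check and remove calls for game, high score and settings data.
; Most functions are thin wrappers over slot-based helpers, alongside getters for cached data and a stored Tutorial value.
; Player save loading and settings saving always use slot 0.
; SaveRivetGameDataToSlot only checks that save data exists without writing it, and the loaded-settings getter returns nothing.
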(fn `GetLoaded SettingsData`
  (returns (SettingsData :type "GameSettingsData Object Reference"))
  (return null))

(fn `GetLoadedHighScoreData`
  (returns (HighScoreRef :type "HighScoreSaveData Object Reference"))
  (return (`self.HighScoreData`)))

(fn `GetLoadedSaveData`
  (returns (SaveGameRef :type "RivetSaveGame Object Reference"))
  (return (`self.SaveGameData`)))

(fn `GetOrLoadOrNewHighScoreData`
  (params (Slot :type Integer))
  (returns (HighScoreDataRef :type "HighScoreSaveData Object Reference"))
  (bind _returnvalue (`self.LoadOrNewHighScoreSaveData` Slot))
  (return _returnvalue))

(fn `GetOrLoadOrNewSaveGameData`
  (params (Slot :type Integer))
  (returns (GameDataRef :type "RivetSaveGame Object Reference"))
  (bind _returnvalue (`self.LoadOrNewGameSaveData` Slot))
  (return _returnvalue))

(fn `GetOrLoadPlayerSaveData`
  (params (Slot :type Integer))
  (returns (SaveData :type "RivetSaveGame Object Reference"))
  (bind _returnvalue (`self.LoadOrNewGameSaveData` 0))
  (return _returnvalue))

(fn `GetOrLoadSettingsData`
  (params (Slot :type Integer))
  (returns (Settings :type "GameSettingsData Object Reference"))
  (bind _returnvalue (`self.LoadOrNewGameSettingsData` Slot))
  (return _returnvalue))

(fn `GetSaveGameData`
  (params (Slot :type Integer))
  (returns (SaveGameDataRef :type "RivetSaveGame Object Reference"))
  (bind _returnvalue (`self.LoadSaveGameFromSlot` Slot))
  (return _returnvalue))

(fn `GetTutorial`
  (returns (TutorialValue :type Boolean))
  (return (`self.Tutorial`)))

(fn `HasHighScoreData`
  (params (Slot :type Integer))
  (returns (HasHighScoreData :type Boolean))
  (bind _returnvalue (`self.DoesHighScoreDataExist` Slot))
  (return _returnvalue))

(fn `HasSaveGameData`
  (params (Slot :type Integer))
  (returns (HasSaveGameData :type Boolean))
  (bind _returnvalue (`self.DoesGameDataExist` Slot))
  (return _returnvalue))

(fn `LoadHighScoreData`
  (params (Slot :type Integer))
  (returns (HighScoreDataRef :type "HighScoreSaveData Object Reference"))
  (bind _returnvalue (`self.LoadHighScoresFromSlot` Slot))
  (return _returnvalue))

(fn `NewGameData`
  (params (Slot :type Integer))
  (returns (GameData :type "RivetSaveGame Object Reference"))
  (bind _returnvalue (`self.CreateNewGameDataAtSlot` Slot))
  (return _returnvalue))

(fn `NewHighScoreData`
  (params (Slot :type Integer))
  (returns (HighScores :type "HighScoreSaveData Object Reference"))
  (bind _returnvalue (`self.CreateNewHighScoreDataAtSlot` Slot))
  (return _returnvalue))

(fn `RemoveRivetGameData`
  (params (Slot :type Integer))
  (returns (Removed :type Boolean))
  (bind _returnvalue (`self.RemoveGameDataFromSlot` Slot))
  (return _returnvalue))

(fn `RemoveRivetHighScoreData`
  (params (Slot :type Integer))
  (returns (Removed :type Boolean))
  (bind _returnvalue (`self.RemoveHighScoreFromSlot` Slot))
  (return _returnvalue))

(fn `RemoveSettingsData`
  (params (SLot :type Integer))
  (returns (RemovedData :type Boolean))
  (bind _returnvalue (`self.RemoveGameSettingsDataFromSlot` SLot))
  (return _returnvalue))

(fn `SaveHighScoreData`
  (params (HighScoreDataRef :type "HighScoreSaveData Object Reference") (Slot :type Integer))
  (`self.SaveHighScoreDataToSlot` HighScoreDataRef Slot))

(fn `SaveRivetGameDataToSlot`
  (params (GameDataRef :type "RivetSaveGame Object Reference") (Slot :type Integer))
  (returns (Saved :type Boolean))
  (bind _hassavegamedata (`self.HasSaveGameData` Slot))
  (return _hassavegamedata))

(fn `SaveSettingsData`
  (params (SaveData :type "GameSettingsData Object Reference"))
  (returns (CouldSave :type Boolean))
  (bind _returnvalue (`self.SaveSettingsDataToSlot` SaveData))
  (return _returnvalue))

(fn `SetTutorial`
  (params (Tutorial :type Boolean))
  (set `self.Tutorial` Tutorial))