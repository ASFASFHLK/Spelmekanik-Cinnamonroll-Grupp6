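; First-person player character for a speedrun shooter, handling Enhanced Input movement, gun fire, GAS dash, emotes and arm-rig animation states.
; Damage triggers camera shake, brief invulnerability, HUD health updates and a one-time critical-health voice line.
; Dynamic materials on the level's PostProcessVolume drive damage, pixelated transition and death glitch effects.
; Save data supplies mouse settings and DT_SkinInfo gun skins, plus a function restoring upgrades, health, position and shop phase.
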(event `self.ReceiveTick`
  (params (DeltaSeconds :type "Float (single-precision)"))
  (bind _asarm_rig_updated_bp (cast `/Game/Animations/Player/new/ArmRigUpdatedBP` (`SkeletalMeshComponent.GetAnimInstance` (`self.RealGun`))))
  (set `/Game/Animations/Player/new/ArmRigUpdatedBP.IsInAir` (`NavMovementComponent.IsFalling` (`self.CharacterMovement`)) _asarm_rig_updated_bp))

(event `self.OnJumped`
  ;[1 1 1] Jump and land events
  (bind _asarm_rig_updated_bp (cast `/Game/Animations/Player/new/ArmRigUpdatedBP` (`SkeletalMeshComponent.GetAnimInstance` (`self.RealGun`))))
  (`FMODBlueprintStatics.PlayEvent2D` "/Game/FMOD/Events/SFX/Player/Player_Jump.Player_Jump")
  (set `/Game/Animations/Player/new/ArmRigUpdatedBP.IsJumping` true _asarm_rig_updated_bp)
  (`KismetSystemLibrary.Delay` 0.2)
  (set `/Game/Animations/Player/new/ArmRigUpdatedBP.IsJumping` false _asarm_rig_updated_bp))

(event `self.OnLanded`
  (params (Hit :type "HitResult Structure (by ref)"))
  ;[1 1 1] Jump and land events
  (bind _asarm_rig_updated_bp (cast `/Game/Animations/Player/new/ArmRigUpdatedBP` (`SkeletalMeshComponent.GetAnimInstance` (`self.RealGun`))))
  (`FMODBlueprintStatics.PlayEvent2D` "/Game/FMOD/Events/SFX/Player/Player_Land.Player_Land")
  (set `/Game/Animations/Player/new/ArmRigUpdatedBP.IsLanding` true _asarm_rig_updated_bp)
  (`KismetSystemLibrary.Delay` 0.2)
  (set `/Game/Animations/Player/new/ArmRigUpdatedBP.IsLanding` false _asarm_rig_updated_bp))

(event `EnhancedInput|/Game/FirstPerson/Input/Actions/IA_Inspect`
  (params (ActionValue :type Boolean) (ElapsedSeconds :type "Float (double-precision)") (TriggeredSeconds :type "Float (double-precision)") (InputAction :type "InputAction Object Reference" :default "/Game/FirstPerson/Input/Actions/IA_Inspect.IA_Inspect"))
  ;[1 1 1] Inspect Weapon
  (:`Triggered`
    (bind _asarm_rig_updated_bp (cast `/Game/Animations/Player/new/ArmRigUpdatedBP` (`SkeletalMeshComponent.GetAnimInstance` (`self.RealGun`))))
    (set `/Game/Animations/Player/new/ArmRigUpdatedBP.IsInspecting` true _asarm_rig_updated_bp)
    (`KismetSystemLibrary.Delay` 0.2)
    (set `/Game/Animations/Player/new/ArmRigUpdatedBP.IsInspecting` false _asarm_rig_updated_bp)))

(event `EnhancedInput|/Game/InputAction/IA_DebugStartShop`
  (params (ActionValue :type Boolean) (ElapsedSeconds :type "Float (double-precision)") (TriggeredSeconds :type "Float (double-precision)") (InputAction :type "InputAction Object Reference" :default "/Game/InputAction/IA_DebugStartShop.IA_DebugStartShop")))

(event `EnhancedInput|/Game/FirstPerson/Input/Actions/IA_Emote`
  (params (ActionValue :type Boolean) (ElapsedSeconds :type "Float (double-precision)") (TriggeredSeconds :type "Float (double-precision)") (InputAction :type "InputAction Object Reference" :default "/Game/FirstPerson/Input/Actions/IA_Emote.IA_Emote"))
  ;[1 1 1] Inspect Weapon
  (:`Triggered`
    (if (`self.CanEmote`)
      (set `self.CanEmote` false)
      (`|PlayMontage` (`self.RealGun`) (`KismetArrayLibrary.Array_Random` (`self.EmoteMontages`))
        (:`OnCompleted`
          (set `self.CanEmote` true))
        (:`OnInterrupted`
          (set `self.CanEmote` true))))))

(event `EnhancedInput|/Game/FirstPerson/Input/Actions/IA_Fire`
  (params (ActionValue :type Boolean) (ElapsedSeconds :type "Float (double-precision)") (TriggeredSeconds :type "Float (double-precision)") (InputAction :type "InputAction Object Reference" :default "/Game/FirstPerson/Input/Actions/IA_Fire.IA_Fire"))
  (:`Triggered`
    (`GunBase.Shoot` (`self.Gun`))))

(event `self.ReceiveBeginPlay`
  (bind _savegameref (message `/Game/Blueprints/BPI_GameInstanceInterface.GetLoadedSaveData` (`GameplayStatics.GetGameInstance`)))
  (bind _returnvalue (`RivetSaveGame.GetWeaponSkin` _savegameref))
  (if (not (`KismetStringLibrary.IsEmpty` _returnvalue))
    (`self.ChangeGunSkin` (`KismetStringLibrary.Conv_StringToName` _returnvalue)))
  (set `self.CanEmote` true)
  (bind _asplayer_controller (cast `PlayerController` (`self.GetController`)))
  (`/Engine/EditorBlueprintResources/StandardMacros.IsValid` _asplayer_controller
    (:`Is Valid`
      (message `EnhancedInputSubsystemInterface.AddMappingContext` _asplayer_controller "/Game/FirstPerson/Input/IMC_Default.IMC_Default" 0 (struct))
      (`self.SetPlayerSettings`)
      (set `self.GunImpactColor` (`KismetMathLibrary.MakeColor` 0.0 22.847843 50.0))
      (`KismetSystemLibrary.Delay` 0.1)
      (`self.InitScreenEffects`)
      (bind _output_get (`self.CreateFadeEffect`))
      (`/Game/Widgets/MainMenu/WBP_BlackScreen.PlayFadeOut` _output_get)
      (bind _effectinstance (`self.SetScreenTransActive`))
      (`self.InitPlayerHealthBar`)
      (bind (_direction _scalevalue) (`Timeline|Timeline` :`NewTime` 1.0 :!via `ReverseFromEnd`)
        (:`Update`
          (`MaterialInstanceDynamic.SetScalarParameterValue` _effectinstance "Pixels" _scalevalue))
        (:`Finished`
          (`PostProcessVolume.AddOrUpdateBlendable` (`self.PostProcessObjecte`) _effectinstance 0.0)
          (`Widget.SetVisibility` (`self.BlackScreenFade`) "Hidden"))))))

(event `self.OnTakeDamage`
  ;[1 1 1] Take damage
  (`self.SetDamageEventActive`)
  (`PlayerCameraManager.StartCameraShake` :`self` (`GameplayStatics.GetPlayerCameraManager` 0) :`ShakeClass` "/Game/Blueprints/DamageCamerShake.DamageCamerShake_C" :`Scale` 10.0 :`PlaySpace` "World")
  (`FMODBlueprintStatics.PlayEvent2D` "/Game/FMOD/Events/SFX/Player/Player_Hit.Player_Hit")
  (`self.UpdateHealthBar`)
  (`self.InvulnerableTimer`)
  (if (<= (`HealthComp.GetHealthPercentage` (`self.HealthComp`)) 0.3)
    (`self.HealthUnder30%`))
  (`|PlayMontage` (`self.RealGun`) "/Game/Animations/Player/new/Animations/ArmDamage_Montage.ArmDamage_Montage"
    (:`then`
      (bind (_direction _damageeffect) (`Timeline|Damage Effect` :`NewTime` 0.2 :!via `PlayFromStart`)
        (:`Update`
          (`self.SetScalerParamter` "Damage" _damageeffect))))))

(event `EnhancedInput|/Game/FirstPerson/Input/Actions/IA_Escape`
  (params (ActionValue :type Boolean) (ElapsedSeconds :type "Float (double-precision)") (TriggeredSeconds :type "Float (double-precision)") (InputAction :type "InputAction Object Reference" :default "/Game/FirstPerson/Input/Actions/IA_Escape.IA_Escape"))
  ;[1 1 1] Open options menu
  (:`Triggered`
    (if (`self.CanPause`)
      (bind _asbp_default_game_mode (cast `/Game/BP_DefaultGameMode` (`GameplayStatics.GetGameMode`)))
      (`/Game/BP_DefaultGameMode.ShowOptions` _asbp_default_game_mode))))

(event `InvulnerableTimer`
  ;[1 1 1] Take damage
  (`self.SetIsInvulnerable` true)
  (`KismetSystemLibrary.Delay` 0.2)
  (`self.SetIsInvulnerable` false))

(event `HealthUnder30%`
  ;[1 1 1] Take damage
  (if (not (`self.ClinkWarned`))
    (bind _asbp_default_game_mode (cast `/Game/BP_DefaultGameMode` (`GameplayStatics.GetGameMode`)))
    (`/Game/BP_DefaultGameMode.ClinkPlayNewVoiceLine` _asbp_default_game_mode "CriticalHealth")
    (set `self.ClinkWarned` true)))

(event `Trigger ScreenTrans`
  (bind _effectinstance (`self.SetScreenTransActive`))
  (bind (_direction _scalevalue) (`Timeline|Trans Effect` :`NewTime` 1.0 :!via `PlayFromStart`)
    (:`Update`
      (`MaterialInstanceDynamic.SetScalarParameterValue` _effectinstance "Pixels" _scalevalue))
    (:`Finished`
      (`PostProcessVolume.AddOrUpdateBlendable` (`self.PostProcessObjecte`) _effectinstance 0.0))))

(event `Trigger Death Effect`
  (`|PlayMontage` (`self.RealGun`) "/Game/Animations/Player/new/Animations/ArmDeath_Loop_Montage.ArmDeath_Loop_Montage"
    (:`then`
      (`self.SetDeathEffectActive`))))

(event `EnhancedInput|/Game/FirstPerson/Input/Actions/IA_Move`
  (params (ActionValue :type "Vector2D Structure") (ElapsedSeconds :type "Float (double-precision)") (TriggeredSeconds :type "Float (double-precision)") (InputAction :type "InputAction Object Reference" :default "/Game/FirstPerson/Input/Actions/IA_Move.IA_Move"))
  (:`Triggered`
    (`self.MoveForward` ActionValue_Y)
    (`self.MoveSides` ActionValue_X)))

(event `EnhancedInput|/Game/FirstPerson/Input/Actions/IA_Jump`
  (params (ActionValue :type Boolean) (ElapsedSeconds :type "Float (double-precision)") (TriggeredSeconds :type "Float (double-precision)") (InputAction :type "InputAction Object Reference" :default "/Game/FirstPerson/Input/Actions/IA_Jump.IA_Jump"))
  (:`Triggered`
    (`self.Jump`))
  (:`Completed`
    (`self.StopJumping`)))

(event `EnhancedInput|/Game/FirstPerson/Input/Actions/IA_Dash`
  (params (ActionValue :type Boolean) (ElapsedSeconds :type "Float (double-precision)") (TriggeredSeconds :type "Float (double-precision)") (InputAction :type "InputAction Object Reference" :default "/Game/FirstPerson/Input/Actions/IA_Dash.IA_Dash"))
  (:`Triggered`
    (`AbilitySystemComponent.TryActivateAbilityByClass` (`AbilitySystemBlueprintLibrary.GetAbilitySystemComponent` null) "/Game/Blueprints/AbilitySystem/BP_DashAbility.BP_DashAbility_C" true)))

(event `self.OnStartupGameplayAbilitiesFinish`)

(event `self.DashVisuals`
  ;[1 1 1] Dash visual
  (`ActorComponent.Activate` (`self.NS_Dash1`) false)
  (`FMODBlueprintStatics.PlayEvent2D` "/Game/FMOD/Events/SFX/Player/Player_Dash.Player_Dash"))

(event `self.ChangeGunSkin`
  (params (SkinName :type Name))
  ;[1 1 1] Change skin
  (bind _savegameref (message `/Game/Blueprints/BPI_GameInstanceInterface.GetLoadedSaveData` (`GameplayStatics.GetGameInstance`)))
  (`RivetSaveGame.SetWeaponSkin` _savegameref (`KismetStringLibrary.Conv_NameToString` SkinName))
  (bind _returnvalue (`|GetDataTableRow` "/Game/Skins/DT_SkinInfo.DT_SkinInfo" SkinName)
    (:`then`
      (bind (_animastion _muzzlecolor _material _unlockround _canbeunlocked _confetti) (break `/Game/Skins/F_SkinStruct` _returnvalue))
      (`PrimitiveComponent.SetMaterial` (`self.RealGun`) 0 _material)
      (`FXSystemComponent.SetColorParameter` (`self.NS_MuzzleFlash`) "Color" _muzzlecolor)
      (`LightComponent.SetLightColor` (`self.PointLight`) _muzzlecolor true)
      (set `self.ShootMontageToPlay` _animastion)
      (set `self.GunImpactColor` _muzzlecolor)
      (if _confetti
        (`ActorComponent.Activate` (`self.NS_Confetti`) false)
        (else
          (`ActorComponent.Deactivate` (`self.NS_Confetti`)))))))

(fn `CreateDeathEffect`
  (bind _returnvalue (`KismetMaterialLibrary.CreateDynamicMaterialInstance` "/Game/Assets/PostProcessMaterials/PP_DeathGlitch.PP_DeathGlitch"))
  (bind _output_get (set `self.DeathEffect` _returnvalue))
  (`PostProcessVolume.AddOrUpdateBlendable` (`self.PostProcessObjecte`) _output_get 0.0))

(fn `CreateFadeEffect`
  (returns (Output_Get :type "/Game/Widgets/MainMenu/WBP_BlackScreen Object Reference"))
  (bind _returnvalue (`|CreateWidget` "/Game/Widgets/MainMenu/WBP_BlackScreen.WBP_BlackScreen_C"))
  (bind _output_get (set `self.BlackScreenFade` _returnvalue))
  (`UserWidget.AddToViewport` _output_get 0)
  (return _output_get))

(fn `CreatePostDamageEffect`
  (bind _returnvalue (`KismetMaterialLibrary.CreateDynamicMaterialInstance` "/Game/Assets/PostProcessMaterials/PP_Damage.PP_Damage"))
  (bind _output_get (set `self.PostDamage` _returnvalue))
  (bind _returnvalue_2 (`GameplayStatics.GetActorOfClass` "/Script/Engine.PostProcessVolume"))
  (bind _output_get_2 (set `self.PostProcessObjecte` _returnvalue_2))
  (`PostProcessVolume.AddOrUpdateBlendable` _output_get_2 _output_get 1.0)
  (`self.SetScalerParamter` "Damage" 2.0))

(fn `CreateScreenTransMaterial`
  (bind _returnvalue (`KismetMaterialLibrary.CreateDynamicMaterialInstance` "/Game/Assets/PostProcessMaterials/PP_Pixelated.PP_Pixelated"))
  (bind _output_get (set `self.PixiliatedScreenMaterial` _returnvalue))
  (if (not (`KismetSystemLibrary.IsValid` (`self.PostProcessObjecte`)))
    (bind _returnvalue_2 (`GameplayStatics.GetActorOfClass` "/Script/Engine.PostProcessVolume"))
    (bind _output_get_2 (set `self.PostProcessObjecte` _returnvalue_2)))
  (`PostProcessVolume.AddOrUpdateBlendable` _output_get_2 _output_get 0.0)
  (`PostProcessVolume.AddOrUpdateBlendable` (`self.PostProcessObjecte`) _output_get 0.0))

(fn `GetMuzzleFlash`
  (returns (NewParam :type Boolean))
  (return false))

(fn `GetPlayerCurrentHealth`
  (returns (Health :type Integer))
  (return (`HealthComp.GetCurrentHealth` (`self.HealthComp`))))

(fn `GetPlayerHud`
  (returns (PlayerHud :type "/Game/Blueprints/Widgets/WB_HUD Object Reference"))
  (return (`self.HudRef`)))

(fn `GetPlayerMaxHealth`
  (returns (MaxHealth :type Integer))
  (return (`HealthComp.GetMaxHealth` (`self.HealthComp`))))

(fn `InitPlayerHealthBar`
  (bind _asbp_hud_class (cast `/Game/Blueprints/BP_HudClass` (`PlayerController.GetHUD` (`GameplayStatics.GetPlayerController` 0))))
  (set `self.HudRef` (`/Game/Blueprints/BP_HudClass.Ui_ref` _asbp_hud_class))
  (`self.SetMaxHealth`)
  (`self.UpdateHealthBar`))

(fn `InitScreenEffects`
  (`self.CreatePostDamageEffect`)
  (`self.CreateScreenTransMaterial`)
  (`self.CreateDeathEffect`))

(fn `Load Saved Game Data`
  (locals (ShopRef :type "/Game/Widgets/Shop/WBP_Shop_New Object Reference"))
  (bind _returnvalue (`GameplayStatics.GetPlayerController` 0))
  (bind _shopref (`local.ShopRef`))
  (bind _gamedataref (message `/Game/Blueprints/BPI_GameInstanceInterface.GetOrLoadOrNewSaveGameData` (`GameplayStatics.GetGameInstance`) 0))
  (bind (_currenthealth _currentcredits _currentround _boughtupgradeslots _worldpos _characterrotator _upgrades) (break `SaveGameData` (`RivetSaveGame.SaveData` _gamedataref)))
  (if (> _currentcredits 1)
    (bind _shopref_2 (message `/Game/Blueprints/BPI_GameModeInterface.GetShopRef` (`GameplayStatics.GetGameMode`)))
    (bind _output_get (set `local.ShopRef` _shopref_2))
    (`/Game/Widgets/Shop/WBP_Shop_New.CreateBoughtSlots` _output_get _boughtupgradeslots)
    (for _array_element _upgrades
      (bind _returnvalue_2 (`|GetDataTableRow` "/Game/Blueprints/AbilitySystem/DT_AbilityTable.DT_AbilityTable" (`KismetStringLibrary.Conv_StringToName` _array_element))
        (:`then`
          (bind _returnvalue_3 (`self.AddPassiveEffect` (`.Ability_23_8032C8F645A3CC283E33C8886721284D` (break `/Game/Blueprints/AbilitySystem/F_AbilityInfo` _returnvalue_2))))
          (`/Game/Widgets/Shop/WBP_Shop_New.CreateSavedBoughtItem` (`local.ShopRef`) (`KismetStringLibrary.Conv_StringToName` _array_element) _returnvalue_3 _returnvalue_2))
        (:`RowNotFound`
          (`KismetSystemLibrary.PrintString` "Ability Not Found"))))
    (`self.UpdateVariables`)
    (set `HealthComp.CurrentHealth` _currenthealth (`self.HealthComp`))
    (`self.K2_TeleportTo` self _worldpos _characterrotator)
    (`self.DisableInput` (`GameplayStatics.GetPlayerPawn` 0) (`GameplayStatics.GetPlayerController` 0))
    (`/Game/Widgets/Shop/WBP_Shop_New.StartShopPhase` _shopref)
    (`Widget.SetVisibility` _shopref "Visible")
    (set `PlayerController.bShowMouseCursor` true _returnvalue)
    (bind _asbp_hud_class (cast `/Game/Blueprints/BP_HudClass` (`PlayerController.GetHUD` _returnvalue)))
    (bind _ui_ref (`/Game/Blueprints/BP_HudClass.Ui_ref` _asbp_hud_class))
    (`/Game/Blueprints/Widgets/WB_HUD.Activate Rounds Visually` _ui_ref _currentround)
    (`Widget.SetVisibility` _ui_ref "Hidden")
    (else
      (`KismetSystemLibrary.PrintString` "New SaveData"))))

(fn `PlayWeaponEffect`
  (bind _returnvalue (`SkeletalMeshComponent.GetAnimInstance` (`self.RealGun`)))
  (`ActorComponent.Activate` (`self.NS_MuzzleFlash`) false)
  (`FMODBlueprintStatics.PlayEvent2D` "/Game/FMOD/Events/SFX/Player/Player_Gunshot.Player_Gunshot")
  (cast `/Game/Animations/Player/new/ArmRigUpdatedBP` _returnvalue)
  (`AnimInstance.Montage_Play` _returnvalue (`self.ShootMontageToPlay`) 1.0 "MontageLength" 0.0 true))

(fn `ResetLoop`
  (set `self.DamageTaken` false)
  (set `self.Damage` 0.0))

(fn `SetDamageEventActive`
  (bind _postdamage (`self.SetScalerParamter` "Loop" 0.1))
  (`PostProcessVolume.AddOrUpdateBlendable` (`self.PostProcessObjecte`) _postdamage 1.0)
  (set `self.DamageTaken` true))

(fn `SetDamageValue`
  (params (Adder :type "Float (double-precision)"))
  (returns (`Value Of Damage` :type "Float (double-precision)"))
  (bind _output_get (set `self.Damage` (+ (`self.Damage`) Adder)))
  (`KismetSystemLibrary.PrintString` (`KismetStringLibrary.Conv_DoubleToString` _output_get))
  (return _output_get))

(fn `SetDeathEffectActive`
  (`PostProcessVolume.AddOrUpdateBlendable` (`self.PostProcessObjecte`) (`self.DeathEffect`) 1.0)
  (`FMODBlueprintStatics.BusStopAllEvents` "/Game/FMOD/Buses/Master/Music.Music" "ALLOWFADEOUT")
  (`FMODBlueprintStatics.BusStopAllEvents` "/Game/FMOD/Buses/Master/SFX.SFX" "ALLOWFADEOUT")
  (`FMODBlueprintStatics.PlayEvent2D` "/Game/FMOD/Events/Music/Stingers/Stinger_PlayerDeath.Stinger_PlayerDeath"))

(fn `SetMaxHealth`
  (`/Game/Blueprints/Widgets/WB_HUD.UpdateMaxHealth` (`self.HudRef`) (`HealthComp.GetMaxHealth` (`self.HealthComp`))))

(fn `SetPlayerSettings`
  (bind _settings (message `/Game/Blueprints/BPI_GameInstanceInterface.GetOrLoadSettingsData` (`GameplayStatics.GetGameInstance`) 0))
  (bind _mousesense (`GameSettingsData.MouseSense` _settings))
  (`self.SetLookUpSpeed` _mousesense)
  (`self.SetLookSidesSpeed` _mousesense)
  (`self.SetMouseInverted` (`GameSettingsData.InvertedMouse` _settings)))

(fn `SetScalerParamter`
  (params (`Scalar param Name` :type Name) (Value :type "Float (double-precision)"))
  (returns (PostDamage :type "MaterialInstanceDynamic Object Reference"))
  (`MaterialInstanceDynamic.SetScalarParameterValue` (`self.PostDamage`) `Scalar param Name` Value)
  (return null))

(fn `SetScreenTransActive`
  (returns (EffectInstance :type "MaterialInstanceDynamic Object Reference"))
  (bind _pixiliatedscreenmaterial (`self.PixiliatedScreenMaterial`))
  (`MaterialInstanceDynamic.SetScalarParameterValue` _pixiliatedscreenmaterial "Pixels" 5.0)
  (`PostProcessVolume.AddOrUpdateBlendable` (`self.PostProcessObjecte`) _pixiliatedscreenmaterial 1.0)
  (return _pixiliatedscreenmaterial))

(fn `SetTimer`
  (params (B :type "Float (double-precision)"))
  (returns (Output_Get :type "Float (double-precision)"))
  (bind _output_get (set `self.TImer` (+ B (`self.TImer`))))
  (return _output_get))

(fn `TakeDamageStart`
  (bind _postdamage (`self.SetScalerParamter` "Loop" 0.1))
  (`PostProcessVolume.AddOrUpdateBlendable` (`self.PostProcessObjecte`) _postdamage 1.0)
  (set `self.DamageTaken` true))

(fn `Update Enemies To Kill`
  (params (`Enemies killed` :type Integer) (`Total enemies` :type Integer))
  (`/Game/Blueprints/Widgets/WB_HUD.Update Enemies` (`self.HudRef`) `Enemies killed` `Total enemies`))

(fn `UpdateHealthBar`
  (bind _hudref (`self.HudRef`))
  (bind _healthcomp (`self.HealthComp`))
  (`/Game/Blueprints/Widgets/WB_HUD.UpdateCurrentHealth` _hudref (`HealthComp.GetCurrentHealth` _healthcomp))
  (`/Game/Blueprints/Widgets/WB_HUD.UpdateHealthBar` _hudref (`HealthComp.GetHealthPercentage` _healthcomp)))

(fn `UserConstructionScript`)