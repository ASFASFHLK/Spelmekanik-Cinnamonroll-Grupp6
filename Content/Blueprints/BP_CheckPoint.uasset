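; BP_CheckPoint is a speedrun checkpoint that reacts to respawn point events with Niagara effects and game mode UI updates.
; When set, it activates its ring effect after a zero-length delay, then has BP_SpeedRunMode show a respawn notification and update the checkpoint count text.
; If all points are checked, the game mode shows the win screen.
; Disabling deactivates the ring, and respawning plays a teleport effect.
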(event `self.RespawnPointDisabled`
  (`ActorComponent.Deactivate` (`self.NS_Ring`)))

(event `self.RespawnPointSet`
  (`KismetSystemLibrary.Delay` 0.0)
  (`ActorComponent.Activate` (`self.NS_Ring`) false)
  (bind _asbp_speed_run_mode (cast `/Game/Blueprints/BP_SpeedRunMode` (`GameplayStatics.GetGameMode`)))
  (`/Game/Blueprints/BP_SpeedRunMode.ShowRespawnNotificatsion` _asbp_speed_run_mode)
  (`/Game/Blueprints/BP_SpeedRunMode.SetCheckpointsText` _asbp_speed_run_mode (`self.GetAmountCheckPointsAsText`))
  (if (`self.HasCheckedAllPoints`)
    (bind _asbp_speed_run_mode_2 (cast `/Game/Blueprints/BP_SpeedRunMode` (`GameplayStatics.GetGameMode`)))
    (`/Game/Blueprints/BP_SpeedRunMode.ShowWinScreen` _asbp_speed_run_mode_2)))

(event `self.RespawnEvent`
  (`ActorComponent.Activate` (`self.NS_Teleport`) false))

(fn `UserConstructionScript`)