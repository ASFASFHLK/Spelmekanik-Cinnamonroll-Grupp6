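; Pooled gorilla melee enemy that slams the ground for radial damage and spawns or throws explosive enemies at the player.
; The slam montage's notify applies damage and Niagara VFX and clears the IsAttacking blackboard key, while spawns are squad-gated and throws launch the partner on an arc.
; Hits flash an overlay and update a Health material parameter.
; Pool spawn and death toggle AI logic around dissolve timelines, with death also triggering a beat-timed music stinger.
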(event `self.SlamIntoGround`
  (bind _returnvalue (`self.GetAttackPointLocation`))
  ;[1 1 1] Create area damage in front
  (`BlackboardComponent.SetValueAsBool` (`self.MyBlackBoard`) "IsAttacking" true)
  (`|PlayMontage` (`self.Mesh`) "/Game/Animations/Gorilla/Animations/GorillaAttack_Montage.GorillaAttack_Montage"
    (:`then`
      (`FMODAudioComponent.Play` (`self.FMOD_Slam`)))
    (:`OnNotifyBegin`
      (if (`self.GetIsAlive`)
        (`GameplayStatics.ApplyRadialDamage` :`BaseDamage` (`self.GetDamage`) :`Origin` _returnvalue :`DamageRadius` 200.0 :`DamageTypeClass` "/Script/Engine.DamageType" :`DamageCauser` self :`InstigatedByController` (`self.GetController`) :`bDoFullDamage` true)
        (`NiagaraFunctionLibrary.SpawnSystemAtLocation` "/Game/Assets/NiagaraSystems/NS_MaugaSlam.NS_MaugaSlam" _returnvalue (struct) (1.0 1.0 1.0) true true "AutoRelease")
        (`BlackboardComponent.SetValueAsBool` (`self.MyBlackBoard`) "IsAttacking" false)))))

(event `KillOnBeat`
  (if (>= (`ReactionalPlaybackLibrary.MusicSystem_GetTimeToBeat` 1.0) 0.5)
    (`ReactionalPlaybackLibrary.Theme_TriggerStinger_Quant` "KillOnBeat" "Instant")))

(event `self.TakeDamageVisual`
  ;[1 1 1] Take damage visually
  (`MeshComponent.SetScalarParameterValueOnMaterials` (`self.Mesh`) "Health" (`HealthComp.GetHealthPercentage` (`self.HealthComp`)))
  (`MeshComponent.SetOverlayMaterial` (`self.Mesh`) "/Game/Assets/Shaders/Material_Instances/Hit_Overlay_Instances/M_Hitoverlay_Inst_Gorilla.M_Hitoverlay_Inst_Gorilla")
  (`KismetSystemLibrary.Delay` 0.05)
  (`FMODBlueprintStatics.PlayEvent2D` "/Game/FMOD/Events/SFX/Player/Player_Gunshot_EnemyHit.Player_Gunshot_EnemyHit")
  (`KismetSystemLibrary.Delay` 0.05)
  (`MeshComponent.SetOverlayMaterial` (`self.Mesh`) "/Engine/Engine_MI_Shaders/Instances/M_Shader_SimpleTranslucent_Invis.M_Shader_SimpleTranslucent_Invis"))

(event `self.Ragdoll`
  (bind _mesh (`self.Mesh`))
  ;[1 1 1] Ragdoll
  (`self.KillOnBeat`)
  (`PrimitiveComponent.SetCollisionEnabled` (`self.CapsuleComponent`) "NoCollision")
  (bind _brain_component (`self.GetBrain`))
  (`BrainComponent.StopLogic` _brain_component "")
  (`FMODAudioComponent.Stop` (`self.FMOD_Slam`))
  (`FMODAudioComponent.Play` (`self.FMOD_Death`))
  (`PrimitiveComponent.SetMaterial` _mesh 0 "/Game/VFX_MayBeDeleted/Dissolve/M_Dissolve_Gorilla.M_Dissolve_Gorilla")
  (bind (_direction _dissolve) (`Timeline|Timeline` :!via `PlayFromStart`)
    (:`Update`
      (`MeshComponent.SetScalarParameterValueOnMaterials` _mesh "Dissolve" _dissolve))
    (:`Finished`
      (`ObjectPooler.ReturnToPool` (subsystem `ObjectPooler`) self))))

(event `self.ThrowExplosiveEnemy`
  (bind _returnvalue (`self.GetPartner`))
  ;[1 1 1] Throw
  (if (`KismetSystemLibrary.IsValid` _returnvalue)
    (`MovementComponent.StopMovementImmediately` (`Character.CharacterMovement` _returnvalue))
    (bind _asbp_explosive_enemy (cast `/Game/EnemyAI/ExplosiveEnemy/BP_ExplosiveEnemy` _returnvalue))
    (`ExplosiveEnemy.SetIsBeingThrown` _asbp_explosive_enemy true)
    (`KismetSystemLibrary.Delay` 0.2)
    (bind _outlaunchvelocity (`GameplayStatics.SuggestProjectileVelocity_CustomArc` (`self.K2_GetActorLocation` _returnvalue) (`self.K2_GetActorLocation` (`GameplayStatics.GetPlayerCharacter` 0)) 0.0 0.6))
    (`self.LaunchCharacter` (`self.GetPartner`) _outlaunchvelocity true true)))

(event `self.SpawnExplosiveEnemy`
  ;[1 1 1] Spawn explosive enemy
  (for _ (range 1 (+ (`self.AmountOfExplosivesToSpawn`) 1))
    (bind _returnvalue (`Squad.CanSpawnExplosive` (`self.MySquad`)))
    (if _returnvalue
      ;[1 1 1] Play animation
      (bind _asgorilla_bp (cast `/Game/Animations/Gorilla/Animations/GorillaBP` (`SkeletalMeshComponent.GetAnimInstance` (`self.Mesh`))))
      (set `/Game/Animations/Gorilla/Animations/GorillaBP.IsSpawningStar` true _asgorilla_bp)
      (bind _asbp_default_game_mode (cast `/Game/BP_DefaultGameMode` (`GameplayStatics.GetGameMode`)))
      (bind _returnvalue_2 (`DefaultGamemode.GetCalculatedScaling` _asbp_default_game_mode))
      (`Enemy_Spawner.SpawnEnemy` (`self.EnemySpawner`) "/Game/EnemyAI/ExplosiveEnemy/BP_ExplosiveEnemy.BP_ExplosiveEnemy_C" (`SceneComponent.K2_GetComponentLocation` (`self.ExplosiveSpawnPoint`)) (`self.K2_GetActorRotation`) _returnvalue_2)
      (`KismetSystemLibrary.Delay` 0.2)
      (set `/Game/Animations/Gorilla/Animations/GorillaBP.IsSpawningStar` false _asgorilla_bp)))
  (`self.ResetThrowTimer`))

(event `self.SpawnFromPool`
  ;[1 1 1] Spawn and activate logic
  (`self.DecideWhichType`)
  (bind (_direction _dissolve) (`Timeline|Timeline_0` :!via `ReverseFromEnd`)
    (:`Update`
      (`MeshComponent.SetScalarParameterValueOnMaterials` (`self.Mesh`) "Dissolve" _dissolve))
    (:`Finished`
      (bind _brain_component (`self.GetBrain`))
      (`BrainComponent.StartLogic` _brain_component)
      (`self.SetIdleAnimation` false))))

(event `self.ReturnToPool`
  (bind _returnvalue (`self.GetMySquad`))
  ;[1 1 1] Return to pool and reset values
  (`self.ShutDownBehavior`)
  (`BlackboardComponent.SetValueAsBool` (`self.MyBlackBoard`) "IsAttacking" false)
  (`PrimitiveComponent.SetMaterial` (`self.Mesh`) 0 "/Game/Assets/Shaders/Material_Instances/Enemy_Master_Instances/M_Enemy_Gorilla.M_Enemy_Gorilla")
  (`self.ReverseRagdoll`)
  (`self.ResetEnemy`)
  (if (`KismetSystemLibrary.IsValid` _returnvalue)
    (`self.K2_SetActorLocation` (`self.K2_GetActorLocation` _returnvalue) false true)))

(event `self.ShutDownBehavior`
  ;[1 1 1] Stops behavior and movement
  (bind _brain_component (`self.GetBrain`))
  (`BrainComponent.StopLogic` _brain_component "")
  (`MovementComponent.StopMovementImmediately` (`self.CharacterMovement`))
  (`self.SetIdleAnimation` true))

(event `self.ReceiveBeginPlay`
  (`self.SetIdleAnimation` true))

(fn `GetBrain`
  (returns (`Brain Component` :type "BrainComponent Object Reference"))
  (return (`AIController.BrainComponent` (`AIBlueprintHelperLibrary.GetAIController` (`self.GetController`)))))

(fn `InitiateRagdoll`
  (`PrimitiveComponent.SetCollisionEnabled` (`self.CapsuleComponent`) "NoCollision")
  (`PrimitiveComponent.SetSimulatePhysics` (`self.Mesh`) true)
  (`PrimitiveComponent.SetCollisionEnabled` (`self.Mesh`) "PhysicsOnly")
  (bind _brain_component (`self.GetBrain`))
  (`BrainComponent.StopLogic` _brain_component ""))

(fn `ReverseRagdoll`
  (bind _mesh (`self.Mesh`))
  (bind _mesh_2 (`self.Mesh`))
  (`PrimitiveComponent.SetCollisionEnabled` (`self.CapsuleComponent`) "QueryAndPhysics")
  (`PrimitiveComponent.SetSimulatePhysics` _mesh false)
  (`PrimitiveComponent.SetCollisionEnabled` _mesh "NoCollision")
  (`SceneComponent.K2_AttachToComponent` (`self.Mesh`) (`self.CapsuleComponent`) "None" "SnapToTarget" "KeepRelative" "KeepRelative" false)
  ;[1 1 1] Ska ändras när den fått en mesh
  (`SceneComponent.K2_SetRelativeRotation` _mesh_2 (struct :`Yaw` -90.0) false false)
  (`SceneComponent.K2_SetRelativeLocation` _mesh_2 (-43.0 52.0 -143.0) false true))

(fn `SetIdleAnimation`
  (params (IsIdle :type Boolean))
  (bind _asgorilla_bp (cast `/Game/Animations/Gorilla/Animations/GorillaBP` (`SkeletalMeshComponent.GetAnimInstance` (`self.Mesh`))))
  (set `/Game/Animations/Gorilla/Animations/GorillaBP.IsIdle` IsIdle _asgorilla_bp))

(fn `UserConstructionScript`)