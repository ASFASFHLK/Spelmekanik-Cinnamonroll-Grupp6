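; Test player character Blueprint that sets up Enhanced Input and fires on player input.
; BeginPlay adds the default mapping context to its player controller, and the fire action calls Shoot.
; AnyDamage only casts player zero's HUD to BP_HudClass, as the health bar update from HealthComp is left disconnected.
; An unused FireMessage call is also disconnected, noted as needing an equipped gun.
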(event `self.ReceiveBeginPlay`
  (bind _asplayer_controller (cast `PlayerController` (`self.GetController`)))
  (`/Engine/EditorBlueprintResources/StandardMacros.IsValid` _asplayer_controller
    (:`Is Valid`
      (message `EnhancedInputSubsystemInterface.AddMappingContext` _asplayer_controller "/Game/FirstPerson/Input/IMC_Default.IMC_Default" 0 (struct)))))

(event `self.ReceiveAnyDamage`
  (params (Damage :type "Float (single-precision)") (DamageType :type "DamageType Object Reference") (InstigatedBy :type "Controller Object Reference") (DamageCauser :type "Actor Object Reference"))
  (bind _asbp_hud_class (cast `/Game/Blueprints/BP_HudClass` (`PlayerController.GetHUD` (`GameplayStatics.GetPlayerController` 0)))))

(event `EnhancedInput|/Game/FirstPerson/Input/Actions/IA_Fire`
  (params (ActionValue :type Boolean) (ElapsedSeconds :type "Float (double-precision)") (TriggeredSeconds :type "Float (double-precision)") (InputAction :type "InputAction Object Reference" :default "/Game/FirstPerson/Input/Actions/IA_Fire.IA_Fire"))
  (:`Triggered`
    (`self.Shoot`)))

(fn `UserConstructionScript`)