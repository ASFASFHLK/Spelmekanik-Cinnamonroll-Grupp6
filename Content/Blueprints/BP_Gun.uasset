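; BP_Gun is a gun Blueprint that supplies visual feedback for firing and hits, with no trace or damage logic in its graphs.
; BeginPlay caches the player pawn as BP_TestPlayerCharacter.
; GunFired plays that character's weapon effect and HUD crosshair animation, while AnimatedonHit plays the HUD hit effect.
; GunHit spawns a pooled Niagara spark at the shotgun hit location, aligned to the impact normal with a pitch offset.
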(event `self.GunFired`
  (bind _playerref (`self.PlayerRef`))
  (`/Game/Blueprints/BP_TestPlayerCharacter.PlayWeaponEffect` _playerref)
  (`/Game/Blueprints/Widgets/WB_HUD.PlayCroshairAnimastion` (`/Game/Blueprints/BP_TestPlayerCharacter.HudRef` _playerref)))

(event `self.ReceiveBeginPlay`
  (bind _asbp_test_player_character (cast `/Game/Blueprints/BP_TestPlayerCharacter` (`GameplayStatics.GetPlayerPawn` 0)))
  (set `self.PlayerRef` _asbp_test_player_character))

(event `self.GunHit`
  (bind (_shotgunhitresult_bblockinghit _shotgunhitresult_binitialoverlap _shotgunhitresult_time _shotgunhitresult_distance _shotgunhitresult_location _shotgunhitresult_impactpoint _shotgunhitresult_normal _shotgunhitresult_impactnormal) (`GameplayStatics.BreakHitResult` (`self.ShotgunHitResult`)))
  (`NiagaraFunctionLibrary.SpawnSystemAtLocation` "/Game/VFX/NiagaraSystems/NS_ImpactSpark.NS_ImpactSpark" (`self.ShotGunHitLocation`) (`KismetMathLibrary.MakeRotator` (.roll (`KismetMathLibrary.Conv_VectorToRotator` _shotgunhitresult_impactnormal)) (+ (.pitch (`KismetMathLibrary.Conv_VectorToRotator` _shotgunhitresult_impactnormal)) 90.0) (.yaw (`KismetMathLibrary.Conv_VectorToRotator` _shotgunhitresult_impactnormal))) (1.0 1.0 1.0) false true "AutoRelease"))

(event `self.AnimatedOnHit`
  (`/Game/Blueprints/Widgets/WB_HUD.PlayHitEffect` (`/Game/Blueprints/BP_TestPlayerCharacter.HudRef` (`self.PlayerRef`))))

(fn `UserConstructionScript`)