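; Gameplay ability for the player's dash, giving visual and HUD feedback and applying a passive effect to the player.
; On activation it commits the cooldown and calls EndAbility immediately, then triggers the character's dash visuals, plays the HUD dash animation and adds the effect.
; GetPlayerRef lazily caches player 0's pawn as BP_TestPlayerCharacter.
; A DashSpeedBoost tag check is left unconnected and never runs.
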(event `self.K2_ActivateAbility`
  (`self.K2_CommitAbilityCooldown` false)
  (`self.K2_EndAbility`)
  (bind (_playerref _output_get) (`self.GetPlayerRef`))
  (`PlayerCharacter.DashVisuals` _playerref)
  (`PlayerCharacter.DashVisuals` _output_get)
  (`/Game/Blueprints/Widgets/WB_HUD.PlayDashAnim` (`/Game/Blueprints/BP_TestPlayerCharacter.HudRef` _playerref))
  (`BaseCharacter.AddPassiveEffect` (`self.PlayerRef`) (`self.Effect`)))

(event `self.K2_OnEndAbility`
  (params (bWasCancelled :type Boolean)))

(fn `GetPlayerRef`
  (returns (PlayerRef :type "/Game/Blueprints/BP_TestPlayerCharacter Object Reference") (Output_Get :type "/Game/Blueprints/BP_TestPlayerCharacter Object Reference"))
  (if (not (`KismetSystemLibrary.IsValid` (`self.PlayerRef`)))
    (bind _asbp_test_player_character (cast `/Game/Blueprints/BP_TestPlayerCharacter` (`GameplayStatics.GetPlayerPawn` 0))
      (:`then`
        (bind _output_get (set `self.PlayerRef` _asbp_test_player_character)))
      (:`CastFailed`
        _)))
  (return (`self.PlayerRef`) _output_get))