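; Game mode for a round-based arena shooter that runs the scripted tutorial, wave rounds, score screen and shop, and game over.
; Intros and tutorial chain announcer and Clink narrator lines through audio-finished delegates and delays to trigger enemy waves.
; Music uses looped, beat-checked Reactional tracks or FMOD events, with playlist and theme ducked under Clink's lines.
; It also restores saved runs, awards credits, unlocks skins by round and records high scores.
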(event `AudioFinished_TutorialWelcome`
  ;[1 1 1] Tutorial
  ;;[1 1 1] Introduction
  (`KismetSystemLibrary.Delay` 1.0)
  (clear `AudioComponent.OnAudioFinished` (`self.ClinkVoice`))
  (`self.AnnouncerPlayNewVoiceLine` "/Game/Audio/SoundCues/Announcer/CUE_Announcer_GameStart.CUE_Announcer_GameStart")
  (add `AudioComponent.OnAudioFinished` (`self.AnnouncerSpeakers`) (delegate `OnAudioFinished_TutorialAnnouncer`)))

(event `OnAudioFinished_TutorialAnnouncer`
  ;[1 1 1] Tutorial
  ;;[1 1 1] Introduction
  (`FMODBlueprintStatics.PlayEvent2D` "/Game/FMOD/Events/Ambience/Crowd_Cheer.Crowd_Cheer")
  (clear `AudioComponent.OnAudioFinished` (`self.AnnouncerSpeakers`))
  (`KismetSystemLibrary.Delay` 2.0)
  (`self.ClinkPlayNewVoiceLine` "TutorialRoundBegin")
  (add `AudioComponent.OnAudioFinished` (`self.ClinkVoice`) (delegate `OnAudioFinished_TutorialFirstRound`)))

(event `OnAudioFinished_TutorialFirstRound`
  ;[1 1 1] Tutorial
  ;;[1 1 1] Introduction
  (clear `AudioComponent.OnAudioFinished` (`self.ClinkVoice`))
  (`KismetSystemLibrary.Delay` 1.0)
  (`self.AnnouncerPlayNewVoiceLine` "/Game/Audio/SoundCues/Announcer/CUE_Announcer_FirstRound.CUE_Announcer_FirstRound")
  (add `AudioComponent.OnAudioFinished` (`self.AnnouncerSpeakers`) (delegate `OnAudioFinished_TutorialCallEnemies`)))

(event `OnAudioFinished_TutorialCallEnemies`
  ;[1 1 1] Tutorial
  ;;[1 1 1] Introduction
  (clear `AudioComponent.OnAudioFinished` (`self.AnnouncerSpeakers`))
  (`KismetSystemLibrary.Delay` 1.0)
  (`FMODBlueprintStatics.PlayEventAtLocation` "/Game/FMOD/Events/Ambience/Arena_Alarm.Arena_Alarm" (`KismetMathLibrary.Conv_VectorToTransform` (`SceneComponent.K2_GetComponentLocation` (`self.AnnouncerSpeakers`))))
  (if (`RivetGameInstance.ReactionalActivated` (`self.As Bp Rivet Game Instance`))
    (bind _asbp_rivet_game_instance (cast `/Game/Blueprints/Bp_RivetGameInstance` (`GameplayStatics.GetGameInstance`)))
    (`ReactionalPlaybackLibrary.Playlist_PlayTrackByIndex` (`RivetGameInstance.SelectedTrack` _asbp_rivet_game_instance))
    (else
      (`FMODBlueprintStatics.PlayEvent2D` "/Game/FMOD/Events/Music/Cyberswarm.Cyberswarm")))
  (`self.PlayRoundVisualEffect`)
  (`KismetSystemLibrary.Delay` 0.5)
  ;;[1 1 1] First wave with range-enemies
  (`Enemy_Spawner.StartNextCustomWave` (`self.SpawnerRef`) "/Game/EnemyAI/RangeEnemy/BP_RangeEnemy.BP_RangeEnemy_C" 3)
  (set `self.EnemiesToKillInTutorial` 3)
  (set `self.TutorialStep` 1)
  (`KismetSystemLibrary.Delay` 1.0)
  (`self.ClinkPlayNewVoiceLine` "TutorialRolyPoly")
  (`KismetSystemLibrary.Delay` 13.0)
  (bind _ui_ref (`self.GetPlayerHUD`))
  (`/Game/Blueprints/Widgets/WB_HUD.ShowDashTutorial` _ui_ref)
  (`KismetSystemLibrary.Delay` 7.0)
  (`/Game/Blueprints/Widgets/WB_HUD.HideDashTutorial` _ui_ref))

(event `self.StartTutorial`
  ;[1 1 1] Tutorial
  (set `self.TutorialActive` true)
  (switch `int` (`self.TutorialStep`)
    (:`0`
      ;;[1 1 1] Introduction
      (`FMODBlueprintStatics.PlayEvent2D` "/Game/FMOD/Events/Ambience/Crowd_Loop.Crowd_Loop")
      (`KismetSystemLibrary.Delay` 3.0)
      (`self.ClinkPlayNewVoiceLine` "TutorialBegin")
      (add `AudioComponent.OnAudioFinished` (`self.ClinkVoice`) (delegate `AudioFinished_TutorialWelcome`)))
    (:`1`
      ;;[1 1 1] Second wave with explosive enemies
      (`KismetSystemLibrary.Delay` 2.0)
      (`Enemy_Spawner.StartNextCustomWave` (`self.SpawnerRef`) "/Game/EnemyAI/ExplosiveEnemy/BP_ExplosiveEnemy.BP_ExplosiveEnemy_C" 6)
      (set `self.EnemiesToKillInTutorial` 5)
      (set `self.TutorialStep` 2)
      (`KismetSystemLibrary.Delay` 1.0)
      (`self.ClinkPlayNewVoiceLine` "TutorialStar"))
    (:`2`
      ;;[1 1 1] Third wave with melee enemies
      (`KismetSystemLibrary.Delay` 2.0)
      (`Enemy_Spawner.StartNextCustomWave` (`self.SpawnerRef`) "/Game/EnemyAI/MeleeEnemy/BP_MeleeEnemy.BP_MeleeEnemy_C" 2)
      (set `self.EnemiesToKillInTutorial` 2)
      (set `self.TutorialStep` 3)
      (`KismetSystemLibrary.Delay` 1.0)
      (`self.ClinkPlayNewVoiceLine` "TutorialGorilla"))
    (:`3`
      ;;[1 1 1] Cleared tutorial
      (set `self.Tutorial` false)
      (`KismetSystemLibrary.Delay` 1.0)
      (`self.ClinkPlayNewVoiceLine` "TutorialEnd")
      (add `AudioComponent.OnAudioFinished` (`self.ClinkVoice`) (delegate `OnAudioFinished_TutorialEnd`))
      (`KismetSystemLibrary.Delay` 4.0)
      (bind _ui_ref (`self.GetPlayerHUD`))
      (`/Game/Blueprints/Widgets/WB_HUD.ShowChargedShotTutorial` _ui_ref)
      (bind _asbp_test_player_character (cast `/Game/Blueprints/BP_TestPlayerCharacter` (`GameplayStatics.GetPlayerPawn` 0)))
      (`/Game/Blueprints/BP_TestPlayerCharacter.ActivateChargedShot` _asbp_test_player_character)
      (set `self.TutorialActive` false)
      (`KismetSystemLibrary.Delay` 9.0)
      (`/Game/Blueprints/Widgets/WB_HUD.HideChargedShotTutorial` _ui_ref))))

(event `OnAudioFinished_TutorialEnd`
  ;[1 1 1] Tutorial
  ;;[1 1 1] Cleared tutorial
  (`KismetSystemLibrary.Delay` 0.2)
  (clear `AudioComponent.OnAudioFinished` (`self.ClinkVoice`))
  (bind _asbp_test_player_character (cast `/Game/Blueprints/BP_TestPlayerCharacter` (`GameplayStatics.GetPlayerPawn` 0)))
  (`HealthComp.SetHealthToMax` (`BaseCharacter.HealthComp` _asbp_test_player_character))
  (`self.StartRoundGameMode`)
  (message `/Game/Blueprints/BPI_GameInstanceInterface.SetTutorial` (`GameplayStatics.GetGameInstance`) false)
  (bind _asbp_test_player_character_2 (cast `/Game/Blueprints/BP_TestPlayerCharacter` (`GameplayStatics.GetPlayerPawn` 0)))
  (`/Game/Blueprints/BP_TestPlayerCharacter.UpdateHealthBar` _asbp_test_player_character_2))

(event `self.ReceiveTick`
  (params (DeltaSeconds :type "Float (single-precision)"))
  ;[1 1 1] Loop track
  (if (`self.RoundActive`)
    (switch `int` (- (`ReactionalPlaybackLibrary.Playlist_GetTrack`) 1)
      (:`0`
        (if (>= (`ReactionalPlaybackLibrary.Playlist_GetCurrentBeat`) 165.0) :!label _label
          (`ReactionalPlaybackLibrary.Playlist_PlayTrackByIndex` (- (`ReactionalPlaybackLibrary.Playlist_GetTrackID`) 1) :!label _label_2)))
      (:`1`
        (goto _label))
      (:`2`
        (if (>= (`ReactionalPlaybackLibrary.Playlist_GetCurrentBeat`) 120.0)
          (goto _label_2))))))

(event `self.StartRoundGameMode`
  ;[1 1 1] Regular gamemode
  (`KismetSystemLibrary.Delay` 3.0)
  (set `self.RoundActive` true)
  (bind _ui_ref (`self.GetPlayerHUD`))
  (`/Game/Blueprints/Widgets/WB_HUD.Activate Rounds Visually` _ui_ref (`self.RoundAmount`))
  (`self.TriggerNextWaveEvent`))

(event `self.OnSpawnNewWave`
  ;[1 1 1] Regular gamemode
  (`self.UpdateEnemiesToKill`))

(event `self.OnStartNextWave`
  (`self.StartNextWave`)
  (if (`RivetGameInstance.ReactionalActivated` (`self.As Bp Rivet Game Instance`))
    (if (`self.bFirstWave`)
      (bind _asbp_rivet_game_instance (cast `/Game/Blueprints/Bp_RivetGameInstance` (`GameplayStatics.GetGameInstance`)))
      (`ReactionalPlaybackLibrary.Playlist_PlayTrackByIndex` (`RivetGameInstance.SelectedTrack` _asbp_rivet_game_instance))
      (`ReactionalPlaybackLibrary.Theme_SetControl` "Health" 0.0))
    (`ReactionalPlaybackLibrary.Theme_TriggerStinger_Quant` "NextRound" "WholeNote")
    (else
      (`FMODBlueprintStatics.PlayEvent2D` "/Game/FMOD/Events/Music/Cyberswarm.Cyberswarm"))))

(event `self.EnemyDied`
  (`self.UpdateEnemiesToKill`))

(event `self.StartShopPhase`
  (set `self.RoundActive` false)
  (if (`self.bFirstWave`)
    (`FMODBlueprintStatics.PlayEvent2D` "/Game/FMOD/Events/Ambience/Crowd_Cheer.Crowd_Cheer")
    (`KismetSystemLibrary.Delay` 2.0)
    (`self.ClinkPlayNewVoiceLine` "WaveClear")
    (`KismetSystemLibrary.Delay` 2.0)
    (`self.StartNextWave`)
    (set `self.bFirstWave` false)
    (else
      (bind _asbp_test_player_character (cast `/Game/Blueprints/BP_TestPlayerCharacter` (`self.PlayerCharacter`) :!label _label_3))
      (`PlayerCharacter.SetIsInvulnerable` _asbp_test_player_character true)
      ;[1 1 1] Reactional
      (`ReactionalPlaybackLibrary.Playlist_Stop` 0.1)
      (`ReactionalPlaybackLibrary.Theme_Stop`)
      (`Squad.ExplodeAllEnemies` (`self.SquadRef`))
      (bind _creditsearned (`self.AddMoney`))
      (`self.UnlockSkins`)
      (bind _asbp_first_person_player_controller (cast `/Game/FirstPerson/Blueprints/BP_FirstPersonPlayerController` (`GameplayStatics.GetPlayerController` 0)))
      (set `/Game/FirstPerson/Blueprints/BP_FirstPersonPlayerController.In Shop` true _asbp_first_person_player_controller)
      (set `/Game/FirstPerson/Blueprints/BP_FirstPersonPlayerController.In Menu` true _asbp_first_person_player_controller)
      (`self.StartScoreScreen` _creditsearned)
      (set `self.bFirstWave` true)
      (`KismetSystemLibrary.Delay` 2.5)
      (`Widget.SetVisibility` (`self.ScoreScreen`) "Hidden")
      (bind _asbp_test_player_character_2 (cast `/Game/Blueprints/BP_TestPlayerCharacter` (`self.PlayerCharacter`)))
      (`/Game/Blueprints/BP_TestPlayerCharacter.Trigger ScreenTrans` _asbp_test_player_character_2)
      (`FMODBlueprintStatics.PlayEvent2D` "/Game/FMOD/Events/UI/ScreenTransitionStart.ScreenTransitionStart")
      (`KismetSystemLibrary.Delay` 1.0)
      (`/Game/Widgets/WBP_ScoreScreen.StartShop` (`self.ScoreScreen`))
      (`self.DisableInput` (`GameplayStatics.GetPlayerPawn` 0) (`GameplayStatics.GetPlayerController` 0))
      (`self.UpdateRoundCounter`)
      ;[1 1 1] Increase amount of enemies every second round
      (if (== 0 (mod (`self.RoundAmount`) 2))
        (`self.IncreaseAmountOfEnemies` 1)
        (`/Game/Widgets/WBP_ScoreScreen.ActivateGoldenGunWidget` (`self.ScoreScreen`) false "")))))

(event `DebugStart SHop`
  (`self.AddCredits` 60000)
  (goto _label_3))

(event `self.ReceiveBeginPlay`
  (bind _returnvalue (`GameplayStatics.GetGameInstance`))
  (bind _asbp_rivet_game_instance (cast `/Game/Blueprints/Bp_RivetGameInstance` (`GameplayStatics.GetGameInstance`)))
  (set `self.As Bp Rivet Game Instance` _asbp_rivet_game_instance)
  (bind _asbp_first_person_player_controller (cast `/Game/FirstPerson/Blueprints/BP_FirstPersonPlayerController` (`GameplayStatics.GetPlayerController` 0)))
  (set `/Game/FirstPerson/Blueprints/BP_FirstPersonPlayerController.In Menu` false _asbp_first_person_player_controller)
  (bind _tutorialvalue (message `/Game/Blueprints/BPI_GameInstanceInterface.GetTutorial` _returnvalue))
  (set `self.Tutorial` _tutorialvalue)
  (bind _settings (message `/Game/Blueprints/BPI_GameInstanceInterface.GetOrLoadSettingsData` _returnvalue 0))
  (bind _returnvalue_2 (`GameplayStatics.GetActorOfClass` "/Script/Engine.PostProcessVolume"))
  (bind _output_get (set `self.PostProcessor` _returnvalue_2))
  (bind _structout (setmembers `PostProcessSettings` :`StructRef` (`PostProcessVolume.Settings` _output_get) :`AutoExposureBias` (`GameSettingsData.ExposureCompensation` _settings)))
  (set `PostProcessVolume.Settings` _structout _output_get)
  (`WidgetBlueprintLibrary.SetInputMode_GameOnly` (`GameplayStatics.GetPlayerController` 0))
  (`self.SpawnShop&ScoreScreen`)
  (`Widget.SetVisibility` (`self.ShopInstanceNew`) "Hidden")
  (`Widget.SetVisibility` (`self.ScoreScreen`) "Hidden")
  (bind _savedata (message `/Game/Blueprints/BPI_GameInstanceInterface.GetOrLoadPlayerSaveData` (`GameplayStatics.GetGameInstance`) 0))
  (if (> (`.CurrentRound` (break `SaveGameData` (`RivetSaveGame.SaveData` _savedata))) 1)
    (`self.LoadSaveData`)
    (elif (`self.Tutorial`)
      (`self.StartTutorial`)
      (else
        ;[1 0.3073 0.3073] Detta händer även om man continue:ar i main menu och kommer in i shoppen
        (`FMODBlueprintStatics.PlayEvent2D` "/Game/FMOD/Events/Ambience/Crowd_Loop.Crowd_Loop")
        (`KismetSystemLibrary.Delay` 2.0)
        (`self.AnnouncerPlayNewVoiceLine` "/Game/Audio/SoundCues/Announcer/CUE_Announcer_GameStart.CUE_Announcer_GameStart")
        (add `AudioComponent.OnAudioFinished` (`self.AnnouncerSpeakers`) (delegate `OnAudioFInished_AnnouncerGameStart`))))))

(event `OnAudioFInished_AnnouncerGameStart`
  ;[1 0.3073 0.3073] Detta händer även om man continue:ar i main menu och kommer in i shoppen
  (`FMODBlueprintStatics.PlayEvent2D` "/Game/FMOD/Events/Ambience/Crowd_Cheer.Crowd_Cheer")
  (clear `AudioComponent.OnAudioFinished` (`self.AnnouncerSpeakers`))
  (`KismetSystemLibrary.Delay` 2.0)
  (`self.ClinkPlayNewVoiceLine` "GameStart")
  (add `AudioComponent.OnAudioFinished` (`self.ClinkVoice`) (delegate `FirstRoundClinkFinished`)))

(event `FirstRoundClinkFinished`
  ;[1 0.3073 0.3073] Detta händer även om man continue:ar i main menu och kommer in i shoppen
  (`KismetSystemLibrary.Delay` 1.0)
  (clear `AudioComponent.OnAudioFinished` (`self.ClinkVoice`))
  (`self.PlayRoundVisualEffect`)
  (`FMODBlueprintStatics.PlayEventAtLocation` "/Game/FMOD/Events/Ambience/Arena_Alarm.Arena_Alarm" (`KismetMathLibrary.Conv_VectorToTransform` (`SceneComponent.K2_GetComponentLocation` (`self.AnnouncerSpeakers`))))
  (`KismetSystemLibrary.Delay` 0.5)
  (`self.StartRoundGameMode`))

(event `ClinkPlayNewVoiceLine`
  (params (VoiceLineName :type Name))
  (bind _clinkvoice (`self.ClinkVoice`))
  ;[1 1 1] Sound
  (bind _returnvalue (`|GetDataTableRow` "/Game/Narrator/DT_Narrator.DT_Narrator" VoiceLineName)
    (:`then`
      (bind _returnvalue_2 (`FMODBlueprintStatics.PlayEvent2D` "/Game/FMOD/Snapshots/VoiceActive.VoiceActive"))
      (`ReactionalPlaybackLibrary.Playlist_SetVolume` 0.5)
      (`ReactionalPlaybackLibrary.Theme_SetVolume` 0.5)
      (bind _playerhud (message `/Game/Blueprints/BPI_PlayerCharacter.GetPlayerHud` (`GameplayStatics.GetPlayerCharacter` 0)))
      (bind (_icon _voiceline) (break `/Game/Narrator/F_NarratorRow` _returnvalue))
      (`/Game/Blueprints/Widgets/WB_HUD.ShowClink` _playerhud _icon)
      (`AudioComponent.SetSound` _clinkvoice _voiceline)
      (`AudioComponent.Play` _clinkvoice 0.0)
      (add `AudioComponent.OnAudioFinished` _clinkvoice (delegate `OnAudioFinished_ClinkVL`)))))

(event `OnAudioFinished_ClinkVL`
  ;[1 1 1] Sound
  (`FMODBlueprintStatics.EventInstanceStop` (stale `ClinkPlayNewVoiceLine` _returnvalue_2))
  (`ReactionalPlaybackLibrary.Playlist_SetVolume` 1.0)
  (`ReactionalPlaybackLibrary.Theme_SetVolume` 1.0)
  (bind _playerhud (message `/Game/Blueprints/BPI_PlayerCharacter.GetPlayerHud` (`GameplayStatics.GetPlayerCharacter` 0)))
  (`/Game/Blueprints/Widgets/WB_HUD.HideClink` _playerhud))

(event `ClinkStop`
  ;[1 1 1] Sound
  (if (> (`AudioComponent.VolumeMultiplier` (`self.ClinkVoice`)) 0.0)
    (`AudioComponent.Stop` (`self.ClinkVoice`))
    (`GameplayStatics.SpawnSound2D` "/Game/Audio/SoundCues/AI/CUE_Rejected.CUE_Rejected" 1.0 1.0 0.0 null)))

(event `VoiceVolumeChange`
  (params (NewVolume :type "Float (double-precision)"))
  ;[1 1 1] Sound
  (`AudioComponent.SetVolumeMultiplier` (`self.ClinkVoice`) NewVolume)
  (`AudioComponent.SetVolumeMultiplier` (`self.AnnouncerSpeakers`) (* NewVolume 3.0)))

(event `NewRoundVoice`
  ;[1 1 1] Sound
  (`self.AnnouncerPlayNewVoiceLine` "/Game/Audio/SoundCues/Announcer/CUE_Announcer_NewRound.CUE_Announcer_NewRound")
  (add `AudioComponent.OnAudioFinished` (`self.AnnouncerSpeakers`) (delegate `NewRoundAnnouncerFinished`)))

(event `NewRoundClinkFinished`
  ;[1 1 1] Sound
  (`KismetSystemLibrary.Delay` 1.0)
  (clear `AudioComponent.OnAudioFinished` (`self.ClinkVoice`))
  (`self.PlayRoundVisualEffect`)
  (`FMODBlueprintStatics.PlayEventAtLocation` "/Game/FMOD/Events/Ambience/Arena_Alarm.Arena_Alarm" (`KismetMathLibrary.Conv_VectorToTransform` (`SceneComponent.K2_GetComponentLocation` (`self.AnnouncerSpeakers`))))
  (`KismetSystemLibrary.Delay` 0.5)
  (`/Game/Widgets/Shop/WBP_Shop_New.StartNextWaveAfterBreak` (`self.ShopInstanceNew`)))

(event `NewRoundAnnouncerFinished`
  ;[1 1 1] Sound
  (bind _asbp_rivet_game_instance (cast `/Game/Blueprints/Bp_RivetGameInstance` (`GameplayStatics.GetGameInstance`)))
  (if (not (`RivetGameInstance.ReactionalActivated` _asbp_rivet_game_instance))
    (`FMODBlueprintStatics.PlayEvent2D` "/Game/FMOD/Events/Music/Cyberswarm.Cyberswarm"))
  (`FMODBlueprintStatics.PlayEvent2D` "/Game/FMOD/Events/Ambience/Crowd_Cheer.Crowd_Cheer")
  (`KismetSystemLibrary.Delay` 2.0)
  (`self.ClinkPlayNewVoiceLine` "NewRound")
  (add `AudioComponent.OnAudioFinished` (`self.ClinkVoice`) (delegate `NewRoundClinkFinished`)))

(event `AnnouncerPlayNewVoiceLine`
  (params (VoiceLine :type "SoundCue Object Reference"))
  (bind _announcerspeakers (`self.AnnouncerSpeakers`))
  ;[1 1 1] Sound
  (`AudioComponent.SetSound` _announcerspeakers VoiceLine)
  (`AudioComponent.Play` _announcerspeakers 0.0))

(event `PlayRoundVisualEffect`
  (bind (_direction _wavered) (`Timeline|Timeline` :`NewTime` 2.0 :!via `PlayFromStart`)
    (:`Update`
      (for _array_element (`self.HoloGramMaterials`)
        (`MaterialInstanceDynamic.SetScalarParameterValue` _array_element "Wave Red" _wavered)))))

(event `self.EndGameEvent`
  (`Squad.ShutDownAllEnemies` (`self.SquadRef`))
  (`self.RecordHighScoreData`)
  (bind _asbp_test_player_character (cast `/Game/Blueprints/BP_TestPlayerCharacter` (`GameplayStatics.GetPlayerPawn` 0))
    (:`then`
      (`/Game/Blueprints/BP_TestPlayerCharacter.Trigger Death Effect` _asbp_test_player_character)
      (`KismetSystemLibrary.Delay` 0.5))
    (:`CastFailed`
      _))
  (bind _returnvalue (`|CreateWidget` "/Game/Widgets/WBP_LoseScreen.WBP_LoseScreen_C"))
  (`UserWidget.AddToViewport` _returnvalue 0)
  (bind _returnvalue_2 (`GameplayStatics.GetActorOfClass` "/Script/Engine.PostProcessVolume"))
  (set `self.PostProcessor` _returnvalue_2)
  (`self.ClinkStop`)
  (`KismetSystemLibrary.Delay` 1.0)
  (`FMODBlueprintStatics.PlayEvent2D` "/Game/FMOD/Events/Voice/Death.Death"))

(fn `AddMoney`
  (returns (CreditsEarned :type Integer))
  (bind _asbp_test_player_character (cast `/Game/Blueprints/BP_TestPlayerCharacter` (`GameplayStatics.GetPlayerCharacter` 0)))
  (bind _asbp_rivet_game_instance (cast `/Game/Blueprints/Bp_RivetGameInstance` (`GameplayStatics.GetGameInstance`)))
  (bind _returnvalue (`KismetMathLibrary.FTrunc` (* (+ (`.CurrentValue` (break `GameplayAttributeData` (`RivetAttributeSet.ExtraCredits` (`BaseCharacter.GetAttributeSet` _asbp_test_player_character)))) 300.0) (`RivetGameInstance.CreditsScaling` _asbp_rivet_game_instance))))
  (`self.AddCredits` _returnvalue)
  (return _returnvalue))

(fn `DebugShopStart`
  (bind _creditsearned (`self.AddMoney`))
  (`self.AddCredits` 6000)
  (`self.StartScoreScreen` _creditsearned))

(fn `GetCurrentAmountCredits`
  (returns (Credits :type Integer))
  (return (`self.GetAmountOfCredits`)))

(fn `GetCurrentRound`
  (returns (`Current Round` :type Integer))
  (return (`self.RoundAmount`)))

(fn `GetPlayerHUD`
  (returns (Ui_ref :type "/Game/Blueprints/Widgets/WB_HUD Object Reference"))
  (bind _asbp_hud_class (cast `/Game/Blueprints/BP_HudClass` (`PlayerController.GetHUD` (`GameplayStatics.GetPlayerController` 0)))
    (:`then`
      _)
    (:`CastFailed`
      _))
  (return (`/Game/Blueprints/BP_HudClass.Ui_ref` _asbp_hud_class)))

(fn `GetShopRef`
  (returns (ShopRef :type "/Game/Widgets/Shop/WBP_Shop_New Object Reference"))
  (return (`self.ShopInstanceNew`)))

(fn `HideHUDAndPauseGame`
  (bind _ui_ref (`self.GetPlayerHUD`))
  (`Widget.SetVisibility` _ui_ref "Hidden")
  (`self.PauseGame` true))

(fn `LoadSaveData`
  (bind _gamedataref (message `/Game/Blueprints/BPI_GameInstanceInterface.GetOrLoadOrNewSaveGameData` (`GameplayStatics.GetGameInstance`) 0))
  (if true
    (bind (_currenthealth _currentcredits _currentround) (break `SaveGameData` (`RivetSaveGame.SaveData` _gamedataref)))
    (bind _output_get (set `self.RoundAmount` _currentround))
    (`KismetSystemLibrary.PrintString` (`KismetStringLibrary.Conv_IntToString` _output_get))
    (`self.IncreaseAmountOfEnemies` (/ _output_get 2))
    (`self.ResetCredits`)
    (`self.AddCredits` _currentcredits)
    (bind _asbp_test_player_character (cast `/Game/Blueprints/BP_TestPlayerCharacter` (`GameplayStatics.GetPlayerPawn` 0)))
    (`PlayerCharacter.TriggerSetupPlayer` _asbp_test_player_character)))

(fn `PauseGame`
  (params (Value :type Boolean))
  (set `PlayerController.bShowMouseCursor` true (`GameplayStatics.GetPlayerController` 0))
  (`GameplayStatics.SetGamePaused` Value)
  (`FMODAudioComponent.Play` (`self.FMOD_GamePaused`)))

(fn `RecordHighScoreData`
  (bind _returnvalue (`GameplayStatics.GetGameInstance`))
  (bind _returnvalue_2 (`GameplayStatics.GetGameInstance`))
  (if (`self.AddedHighScore`)
    (return)
    (else
      (set `self.AddedHighScore` true)
      (bind _highscoredataref (message `/Game/Blueprints/BPI_GameInstanceInterface.GetOrLoadOrNewHighScoreData` _returnvalue 0))
      (bind _savedata (message `/Game/Blueprints/BPI_GameInstanceInterface.GetOrLoadPlayerSaveData` _returnvalue 0))
      (`HighScoreSaveData.AddHighScoreItem` _highscoredataref (make `HighScoreData` (`KismetTextLibrary.Conv_StringToText` (`.PlayerName` (break `SaveGameData` (`RivetSaveGame.SaveData` _savedata)))) (`self.RoundAmount`) 60.0 (`KismetMathLibrary.Now`)))
      (message `/Game/Blueprints/BPI_GameInstanceInterface.SaveHighScoreData` _returnvalue _highscoredataref 0)
      (message `/Game/Blueprints/BPI_GameInstanceInterface.RemoveRivetGameData` _returnvalue_2 0)
      (bind _settings (message `/Game/Blueprints/BPI_GameInstanceInterface.GetOrLoadSettingsData` _returnvalue_2 0))
      (bind _gamedata (message `/Game/Blueprints/BPI_GameInstanceInterface.NewGameData` _returnvalue_2 0))
      (`RivetSaveGame.SetPlayerName` _gamedata (`GameSettingsData.PlayerName` _settings))
      (message `/Game/Blueprints/BPI_GameInstanceInterface.SaveRivetGameDataToSlot` (`GameplayStatics.GetGameInstance`) _gamedata 0))))

(fn `RegisterHoloGramMaterials`
  (params (`Dynamic Materials` :type "Array of MaterialInstanceDynamic Object Reference"))
  (for _array_element `Dynamic Materials`
    (`KismetArrayLibrary.Array_Add` (`self.HoloGramMaterials`) _array_element)))

(fn `ResumeGame`
  (set `PlayerController.bShowMouseCursor` false (`GameplayStatics.GetPlayerController` 0))
  (`GameplayStatics.SetGamePaused` false)
  (`FMODAudioComponent.Stop` (`self.FMOD_GamePaused`)))

(fn `ShowOptions`
  (bind _optionsinstance (`self.OptionsInstance`))
  (set `Widget.Visibility` "Visible" _optionsinstance)
  (`self.HideHUDAndPauseGame`)
  (`/Game/Widgets/WBP_PauseMenu.PlayFadein` _optionsinstance))

(fn `SpawnShop&ScoreScreen`
  (bind _returnvalue (`|CreateWidget` "/Game/Widgets/WBP_PauseMenu.WBP_PauseMenu_C"))
  (bind _output_get (set `self.OptionsInstance` _returnvalue))
  (`UserWidget.AddToViewport` _output_get 0)
  (`Widget.SetVisibility` (`self.OptionsInstance`) "Hidden")
  (bind _returnvalue_2 (`|CreateWidget` "/Game/Widgets/WBP_ScoreScreen.WBP_ScoreScreen_C"))
  (bind _output_get_2 (set `self.ScoreScreen` _returnvalue_2))
  (`UserWidget.AddToViewport` _output_get_2 0)
  (bind _returnvalue_3 (`|CreateWidget` "/Game/Widgets/Shop/WBP_Shop_New.WBP_Shop_New_C"))
  (bind _output_get_3 (set `self.ShopInstanceNew` _returnvalue_3))
  (`UserWidget.AddToViewport` _output_get_3 0)
  (return))

(fn `StartScoreScreen`
  (params (`Money Made` :type Integer))
  (bind _scorescreen (`self.ScoreScreen`))
  (bind _ui_ref (`self.GetPlayerHUD`))
  (`Widget.SetVisibility` _ui_ref "Hidden")
  (`Widget.SetVisibility` _scorescreen "Visible")
  (`/Game/Widgets/WBP_ScoreScreen.SetMoneyMade` _scorescreen `Money Made`)
  (`FMODBlueprintStatics.BusStopAllEvents` "/Game/FMOD/Buses/Master/Music.Music" "IMMEDIATE")
  (`FMODBlueprintStatics.PlayEvent2D` "/Game/FMOD/Events/Music/Stingers/Stinger_RoundEnd.Stinger_RoundEnd")
  (`FMODBlueprintStatics.PlayEvent2D` "/Game/FMOD/Events/Ambience/Crowd_Cheer.Crowd_Cheer"))

(fn `StartShopScreen`
  (bind _shopinstancenew (`self.ShopInstanceNew`))
  (`Widget.SetVisibility` (`self.ScoreScreen`) "Hidden")
  (`Widget.SetVisibility` _shopinstancenew "Visible")
  (`/Game/Widgets/Shop/WBP_Shop_New.StartShopPhase` _shopinstancenew))

(fn `UnlockSkins`
  (locals (UnlockedSkin :type Boolean))
  (bind _returnvalue (`GameplayStatics.GetGameInstance`))
  (bind _unlockdataref (message `/Game/Blueprints/BPI_GameInstanceInterface.GetOrLoadUnlockData` _returnvalue 0))
  (bind _outrownames (`DataTableFunctionLibrary.GetDataTableRowNames` "/Game/Skins/DT_SkinInfo.DT_SkinInfo"))
  (for _array_element _outrownames
    (bind _returnvalue_2 (`|GetDataTableRow` "/Game/Skins/DT_SkinInfo.DT_SkinInfo" _array_element)
      (:`then`
        (bind (_animastion _muzzlecolor _material _unlockround _canbeunlocked) (break `/Game/Skins/F_SkinStruct` _returnvalue_2))
        (if _canbeunlocked
          (if (== (`self.RoundAmount`) _unlockround)
            (bind _returnvalue_3 (`KismetStringLibrary.Conv_NameToString` _array_element))
            (bind _returnvalue_4 (`RivetUnlockSaveData.HasItem` _unlockdataref _returnvalue_3))
            (if (not _returnvalue_4)
              (`RivetUnlockSaveData.AddUnlockedItem` _unlockdataref _returnvalue_3)
              (`/Game/Widgets/WBP_ScoreScreen.ActivateGoldenGunWidget` (`self.ScoreScreen`) true _returnvalue_3)))))))
  (message `/Game/Blueprints/BPI_GameInstanceInterface.SaveUnlockData` _returnvalue _unlockdataref 0))

(fn `UpdateEnemiesToKill`
  (bind _asbp_test_player_character (cast `/Game/Blueprints/BP_TestPlayerCharacter` (`GameplayStatics.GetPlayerPawn` 0)))
  (`/Game/Blueprints/BP_TestPlayerCharacter.Update Enemies To Kill` _asbp_test_player_character (`self.CurrentAmountKilled`) (`self.AmountToKill`)))

(fn `UpdateRoundCounter`
  (bind _output_get (set `self.RoundAmount` (+ 1 (`self.RoundAmount`))))
  (bind _ui_ref (`self.GetPlayerHUD`))
  (`TextBlock.SetText` (`/Game/Blueprints/Widgets/WB_HUD.RoundCounter` _ui_ref) (`KismetTextLibrary.Conv_IntToText` _output_get)))

(fn `UserConstructionScript`)