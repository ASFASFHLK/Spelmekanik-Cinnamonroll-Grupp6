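; Enemy spawner Blueprint that pulls enemies from an object pool and scales their health and damage.
; SpawnEnemy places a pooled enemy of the given type at a transform, assigns it the squad, and also registers explosive enemies with that squad.
; It caches the player character on BeginPlay so a separate event can push killed and total enemy counts to the player for the kill-progress widget.
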(event `self.UpdateEnemiesToKillWidget`
  ;[1 1 1] Varför ligger denna här och inte i game modet?
  (`/Game/Blueprints/BP_TestPlayerCharacter.Update Enemies To Kill` (`self.Playerref`) (`self.AmountOfEnemiesKilled`) (`self.EnemiesToKill`)))

(event `self.ReceiveBeginPlay`
  (bind _asbp_test_player_character (cast `/Game/Blueprints/BP_TestPlayerCharacter` (`Controller.K2_GetPawn` (`GameplayStatics.GetPlayerController` 0))))
  (set `self.Playerref` _asbp_test_player_character))

(event `self.SpawnEnemy`
  (params (EnemyType :type "BaseEnemy Class Reference") (Location :type "Vector Structure") (Rotation :type "Rotator Structure"))
  ;[1 1 1] Spawn enemy and set scaling
  (bind _spawnedactor (`ObjectPooler.SpawnFromPool` (subsystem `ObjectPooler`) EnemyType Location Rotation))
  (bind _asbp_explosive_enemy (cast `/Game/EnemyAI/ExplosiveEnemy/BP_ExplosiveEnemy` _spawnedactor)
    (:`then`
      (`Squad.AddExplosiveToSquad` (`self.GetSquad`) _asbp_explosive_enemy))
    (:`CastFailed`
      _))
  (`BaseEnemy.SetSquad` _spawnedactor (`self.GetSquad`))
  (`BaseEnemy.ScaleHealthAndDamage` _spawnedactor (`self.ScalingHealth`) (`self.ScalingDamage`)))

(fn `UserConstructionScript`)