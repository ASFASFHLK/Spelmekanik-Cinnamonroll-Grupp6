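; Ranged enemy projectile that launches at the player character and damages it on hit.
; On spawn it takes an arced velocity from SuggestProjectileVelocityCustomArc, then briefly homes on the player after a short delay.
; A mesh hit destroys it, immediately after damaging the player or shortly after striking anything else, with a timed self-destroy as fallback.
; Alternative aiming, impact effect and pool-return nodes are left disconnected.
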(event `self.ReceiveBeginPlay`
  (bind _projectilemovement (`self.ProjectileMovement`))
  (bind _projectilemovement_2 (`self.ProjectileMovement`))
  ;[1 1 1] Shoot projectile at player
  (bind _outlaunchvelocity (`GameplayStatics.SuggestProjectileVelocity_CustomArc` (`self.K2_GetActorLocation`) (`self.K2_GetActorLocation` (`GameplayStatics.GetPlayerCharacter` 0))))
  (set `MovementComponent.Velocity` _outlaunchvelocity _projectilemovement_2)
  (set `ProjectileMovementComponent.bRotationFollowsVelocity` true _projectilemovement_2)
  (`KismetSystemLibrary.Delay` 0.5)
  (set `ProjectileMovementComponent.HomingTargetComponent` (`self.GetComponentByClass` (`GameplayStatics.GetPlayerCharacter` 0) "/Script/Engine.SceneComponent") _projectilemovement)
  (set `ProjectileMovementComponent.bIsHomingProjectile` true _projectilemovement)
  (`KismetSystemLibrary.Delay` 1.5)
  (set `ProjectileMovementComponent.bIsHomingProjectile` false (`self.ProjectileMovement`))
  (`KismetSystemLibrary.Delay` 20.0)
  (`self.K2_DestroyActor`))

(event `self.ProjectileMesh.OnComponentHit`
  (params (HitComponent :type "PrimitiveComponent Object Reference") (OtherActor :type "Actor Object Reference") (OtherComp :type "PrimitiveComponent Object Reference") (NormalImpulse :type "Vector Structure") (Hit :type "HitResult Structure (by ref)"))
  ;[1 1 1] When the projectile hits something
  (bind _asbp_test_player_character (cast `/Game/Blueprints/BP_TestPlayerCharacter` OtherActor)
    (:`then`
      (`self.DealDamage` _asbp_test_player_character))
    (:`CastFailed`
      (`KismetSystemLibrary.Delay` 0.1)))
  (`self.K2_DestroyActor`))

(fn `UserConstructionScript`)