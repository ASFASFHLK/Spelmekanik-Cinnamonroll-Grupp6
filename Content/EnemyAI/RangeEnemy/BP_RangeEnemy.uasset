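; Pooled ranged RolyPoly enemy character that shoots projectiles, with FMOD audio for fight, flight, rolling and death.
; Spawning reverses a dissolve, then starts AI logic; returning resets it and moves it to its squad.
; Despite its name, Ragdoll stops the AI, dissolves the mesh, checks beat timing for a music stinger, then pools the actor.
; Other events handle hit overlay flashes, flee and lock-in sounds, and the attack montage; InitiateRagdoll's physics path is unused.
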(event `self.SpawnFromPool`
  ;[1 1 1] Spawn and activate logic
  (bind (_direction _dissolve) (`Timeline|Timeline` :!via `ReverseFromEnd`)
    (:`Update`
      (`MeshComponent.SetScalarParameterValueOnMaterials` (`self.Mesh`) "Dissolve" _dissolve))
    (:`Finished`
      (bind _brain_component (`self.GetBrain`))
      (`BrainComponent.StartLogic` _brain_component))))

(event `self.ReturnToPool`
  (bind _returnvalue (`self.GetMySquad`))
  ;[1 1 1] Return to pool and reset mesh and stats
  (`self.ReverseRagdoll`)
  (`PrimitiveComponent.SetMaterial` (`self.Mesh`) 0 "/Game/Assets/Shaders/Material_Instances/Enemy_Master_Instances/M_Enemy_RolyPoly.M_Enemy_RolyPoly")
  (`self.ResetEnemy`)
  (if (`KismetSystemLibrary.IsValid` _returnvalue)
    (`self.K2_SetActorLocation` (`self.K2_GetActorLocation` _returnvalue) false true)))

(event `self.TakeDamageVisual`
  ;[1 1 1] Visually take damage
  (`MeshComponent.SetOverlayMaterial` (`self.Mesh`) "/Game/Assets/Shaders/Material_Instances/Hit_Overlay_Instances/M_Hitoverlay_Inst_Roly.M_Hitoverlay_Inst_Roly")
  (`KismetSystemLibrary.Delay` 0.05)
  (`FMODBlueprintStatics.PlayEvent2D` "/Game/FMOD/Events/SFX/Player/Player_Gunshot_EnemyHit.Player_Gunshot_EnemyHit")
  (`KismetSystemLibrary.Delay` 0.05)
  (`MeshComponent.SetOverlayMaterial` (`self.Mesh`) "/Engine/Engine_MI_Shaders/Instances/M_Shader_SimpleTranslucent_Invis.M_Shader_SimpleTranslucent_Invis"))

(event `KillOnBeat`
  (if (>= (`ReactionalPlaybackLibrary.MusicSystem_GetTimeToBeat` 1.0) 0.5)
    (`ReactionalPlaybackLibrary.Theme_TriggerStinger_Quant` "HitOnBeat" "Instant")))

(event `self.Ragdoll`
  ;[1 1 1] Ragdoll
  (`self.KillOnBeat`)
  (`PrimitiveComponent.SetCollisionEnabled` (`self.CapsuleComponent`) "NoCollision")
  (`self.ShutDownBehavior`)
  (`FMODAudioComponent.Play` (`self.FMOD_Death`))
  (`FMODAudioComponent.Stop` (`self.FMOD_Fight`))
  (`FMODAudioComponent.Stop` (`self.FMOD_Flight`))
  (`FMODAudioComponent.Stop` (`self.FMOD_Roll`))
  (`PrimitiveComponent.SetMaterial` (`self.Mesh`) 0 "/Game/VFX_MayBeDeleted/Dissolve/M_Dissolve_Roly.M_Dissolve_Roly")
  (bind (_direction _dissolve) (`Timeline|Dissolver` :!via `PlayFromStart`)
    (:`Update`
      (`MeshComponent.SetScalarParameterValueOnMaterials` (`self.Mesh`) "Dissolve" _dissolve))
    (:`Finished`
      (`ObjectPooler.ReturnToPool` (subsystem `ObjectPooler`) self))))

(event `self.Flee`
  ;[1 1 1] Flyr från spelaren
  (`FMODAudioComponent.Play` (`self.FMOD_Flight`))
  (`KismetSystemLibrary.Delay` 0.5)
  (`FMODAudioComponent.Play` (`self.FMOD_Roll`)))

(event `self.LockInPlace`
  ;[1 1 1] Hittar en position och börjar skjuta
  (`FMODAudioComponent.Play` (`self.FMOD_Fight`))
  (`FMODAudioComponent.Stop` (`self.FMOD_Roll`)))

(event `self.FireProjectile`
  ;[1 1 1] Shoots a projectile
  (`|PlayMontage` (`self.Mesh`) "/Game/Animations/Rolypoly/Animations/RolyAttack_Montage.RolyAttack_Montage"))

(event `self.ShutDownBehavior`
  ;[1 1 1] Stops behavior and movement
  (bind _brain_component (`self.GetBrain`))
  (`BrainComponent.StopLogic` _brain_component "")
  (`MovementComponent.StopMovementImmediately` (`self.CharacterMovement`)))

(fn `GetBrain`
  (returns (`Brain Component` :type "BrainComponent Object Reference"))
  (return (`AIController.BrainComponent` (`AIBlueprintHelperLibrary.GetAIController` (`self.GetController`)))))

(fn `InitiateRagdoll`
  (`PrimitiveComponent.SetCollisionEnabled` (`self.CapsuleComponent`) "NoCollision")
  (`PrimitiveComponent.SetSimulatePhysics` (`self.Mesh`) true)
  (`PrimitiveComponent.SetCollisionEnabled` (`self.Mesh`) "PhysicsOnly")
  (bind _brain_component (`self.GetBrain`))
  (`BrainComponent.StopLogic` _brain_component ""))

(fn `ReverseRagdoll`
  (bind _mesh (`self.Mesh`))
  (bind _mesh_2 (`self.Mesh`))
  (`PrimitiveComponent.SetCollisionEnabled` (`self.CapsuleComponent`) "QueryAndPhysics")
  (`PrimitiveComponent.SetSimulatePhysics` _mesh false)
  (`PrimitiveComponent.SetCollisionEnabled` _mesh "NoCollision")
  (`SceneComponent.K2_AttachToComponent` (`self.Mesh`) (`self.CapsuleComponent`) "None" "SnapToTarget" "KeepRelative" "KeepRelative" false)
  (`SceneComponent.K2_SetRelativeRotation` _mesh_2 (struct :`Yaw` -90.0) false false)
  (`SceneComponent.K2_SetRelativeLocation` _mesh_2 (0.0 0.0 -86.0) false false))

(fn `UserConstructionScript`)