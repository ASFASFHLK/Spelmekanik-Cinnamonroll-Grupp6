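; Jump powerup pickup for a speedrun game mode, reacting to pickup and respawn events with visual effects and UI text.
; On pickup it has BP_SpeedRunMode update stats and show the ability's name and description, then swaps the Niagara ring for a brief pickup burst.
; The ring activates on BeginPlay and respawn.
; The jump boost itself is not implemented in these graphs.
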(event `self.ItemRespawned`
  (`ActorComponent.Activate` (`self.NS_Ring`) false :!label _label))

(event `self.ItemPickedUped`
  (bind _asbp_speed_run_mode (cast `/Game/Blueprints/BP_SpeedRunMode` (`GameplayStatics.GetGameMode`)))
  (`/Game/Blueprints/BP_SpeedRunMode.UpdateStats` _asbp_speed_run_mode)
  (`/Game/Blueprints/BP_SpeedRunMode.SetPickUpText` _asbp_speed_run_mode (`self.NameOfAbility`) (`self.Description`))
  (`KismetSystemLibrary.Delay` 0.0)
  (`ActorComponent.Deactivate` (`self.NS_Ring`))
  (`ActorComponent.Activate` (`self.NS_Pickup`) false)
  (`KismetSystemLibrary.Delay` 0.2)
  (`ActorComponent.Deactivate` (`self.NS_Pickup`)))

(event `self.ReceiveBeginPlay`
  (goto _label))

(fn `UserConstructionScript`)