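; Player explosive projectile that deals full radial damage, sparing the player, on its first hit or overlap.
; On BeginPlay it reads its blast radius from BP_TestPlayerCharacter.
; Hit and overlap share one path, guarded by CanExplode, that applies damage, activates two effect components and plays the charged explosion audio event.
; It then hides the mesh and delays destruction so the effects can play out.
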(event `self.ReceiveHit`
  (params (MyComp :type "PrimitiveComponent Object Reference") (Other :type "Actor Object Reference") (OtherComp :type "PrimitiveComponent Object Reference") (bSelfMoved :type Boolean) (HitLocation :type "Vector Structure") (HitNormal :type "Vector Structure") (NormalImpulse :type "Vector Structure") (Hit :type "HitResult Structure (by ref)"))
  (bind _returnvalue (`self.K2_GetActorLocation`))
  (if (`self.CanExplode`) :!label _label
    (`GameplayStatics.ApplyRadialDamage` (`self.Damage`) _returnvalue (`self.Radius`) null (`|MakeArray` (`GameplayStatics.GetPlayerPawn` 0) :!type "Actor Object Reference") (`self.GetOwner`) (`GameplayStatics.GetPlayerController` 0) true)
    (set `self.CanExplode` false)
    (`ActorComponent.Activate` (`self.NS_Venture`) false)
    (`ActorComponent.Activate` (`self.NS_ExplodeStar`) false)
    (`FMODBlueprintStatics.PlayEventAtLocation` "/Game/FMOD/Events/SFX/Player/Player_ChargedExplosion.Player_ChargedExplosion" (`KismetMathLibrary.Conv_VectorToTransform` _returnvalue))
    (`SceneComponent.SetVisibility` (`self.ProjectileMesh`) false false)
    (`KismetSystemLibrary.Delay` 5.0)
    (`self.K2_DestroyActor`)))

(event `self.ReceiveBeginPlay`
  (bind _asbp_test_player_character (cast `/Game/Blueprints/BP_TestPlayerCharacter` (`GameplayStatics.GetPlayerPawn` 0)))
  (bind _current_value (`/Game/Blueprints/BP_TestPlayerCharacter.GetExplosionRadius` _asbp_test_player_character))
  (set `self.Radius` _current_value))

(event `self.ReceiveActorBeginOverlap`
  (params (OtherActor :type "Actor Object Reference"))
  (goto _label))

(fn `UserConstructionScript`)