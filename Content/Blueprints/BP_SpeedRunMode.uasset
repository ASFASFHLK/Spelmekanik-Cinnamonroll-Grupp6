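; Speedrun mode Blueprint that times the player's run and drives the speedrun overlay and win screen.
; BeginPlay finds the checkpoint kill box as its manager, creates the overlay and fills in checkpoint count and stats after a short delay.
; Tick accumulates elapsed time for the timer, while functions push pickup, checkpoint and respawn notifications.
; A one-shot win screen shows time, falls and grade, hiding the HUD message and overlay.
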(event `self.ReceiveBeginPlay`
  (bind _returnvalue (`GameplayStatics.GetActorOfClass` "/Game/Blueprints/BP_CheckPointKillBox.BP_CheckPointKillBox_C"))
  (set `self.CheckPoint Manager` _returnvalue)
  (bind _returnvalue_2 (`|CreateWidget` "/Game/Blueprints/Widgets/Speedrun/WB_SpeedrunOverlay.WB_SpeedrunOverlay_C"))
  (bind _output_get (set `self.SpeedRunWidget` _returnvalue_2))
  (`UserWidget.AddToViewport` _output_get 0)
  (`KismetSystemLibrary.Delay` 0.2)
  (`self.UpdateStats`)
  (`/Game/Blueprints/Widgets/Speedrun/WB_SpeedrunOverlay.SetAmountOfCheckPoints` (`self.SpeedRunWidget`) (`KismetTextLibrary.Conv_StringToText` (`CheckPointKillBox.GetRoundsAsText` (`self.CheckPoint Manager`)))))

(event `self.ReceiveTick`
  (params (DeltaSeconds :type "Float (single-precision)"))
  (bind _speedrunwidget (`self.SpeedRunWidget`))
  (set `self.Timetaken` (+ DeltaSeconds (`self.Timetaken`)))
  (`parent.ReceiveTick` DeltaSeconds)
  (`/Engine/EditorBlueprintResources/StandardMacros.IsValid` _speedrunwidget
    (:`Is Valid`
      (bind _time_as_text (`self.GetTimeAsText`))
      (`/Game/Blueprints/Widgets/Speedrun/WB_SpeedrunOverlay.UpdateTimer` _speedrunwidget _time_as_text))))

(fn `GetTimeAsText`
  (returns (`Time as text` :type Text))
  (return (`KismetTextLibrary.Conv_DoubleToText` (`self.Timetaken`) "HalfToEven")))

(fn `SetCheckpointsText`
  (params (TotalCheckedPoints :type String))
  (bind _speedrunwidget (`self.SpeedRunWidget`))
  (`/Engine/EditorBlueprintResources/StandardMacros.IsValid` _speedrunwidget
    (:`Is Valid`
      (`/Game/Blueprints/Widgets/Speedrun/WB_SpeedrunOverlay.SetAmountOfCheckPoints` _speedrunwidget (`KismetTextLibrary.Conv_StringToText` TotalCheckedPoints)))))

(fn `SetPickUpText`
  (params (NameOfAbility :type Text) (DescriptsionOfAbility :type Text))
  (bind _speedrunwidget (`self.SpeedRunWidget`))
  (`/Engine/EditorBlueprintResources/StandardMacros.IsValid` _speedrunwidget
    (:`Is Valid`
      (`/Game/Blueprints/Widgets/Speedrun/WB_SpeedrunOverlay.SetPowerupText` _speedrunwidget NameOfAbility DescriptsionOfAbility)
      (`/Game/Blueprints/Widgets/Speedrun/WB_SpeedrunOverlay.ShowNotifcationtext` _speedrunwidget))))

(fn `ShowRespawnNotificatsion`
  (bind _speedrunwidget (`self.SpeedRunWidget`))
  (`/Engine/EditorBlueprintResources/StandardMacros.IsValid` _speedrunwidget
    (:`Is Valid`
      (`/Game/Blueprints/Widgets/Speedrun/WB_SpeedrunOverlay.SetNotifcatsionText` _speedrunwidget "Checkpoint" "Reached" "You will now respawn here")
      (`/Game/Blueprints/Widgets/Speedrun/WB_SpeedrunOverlay.ShowNotifcationtext` _speedrunwidget))))

(fn `ShowWinScreen`
  (locals (NewLocalVar :type "/Game/Widgets/WBP_WinScreen Object Reference"))
  (if (not (`self.ScoreScreenCreated`))
    (set `self.ScoreScreenCreated` true)
    (bind _returnvalue (`|CreateWidget` "/Game/Widgets/WBP_WinScreen.WBP_WinScreen_C"))
    (`UserWidget.AddToViewport` _returnvalue 0)
    (bind _time_as_text (`self.GetTimeAsText`))
    (`/Game/Widgets/WBP_WinScreen.ShowStatsEvent` _returnvalue _time_as_text (`KismetTextLibrary.Conv_IntToText` (`CheckPointKillBox.GetAmountOfRespawns` (`self.CheckPoint Manager`))) (`self.Grade`))
    (bind _playerhud (message `/Game/Blueprints/BPI_PlayerCharacter.GetPlayerHud` (`GameplayStatics.GetPlayerCharacter` 0)))
    (`Widget.SetVisibility` _playerhud "Hidden")
    (`Widget.SetVisibility` (`self.SpeedRunWidget`) "Hidden")))

(fn `UpdateStats`
  (bind _speedrunwidget (`self.SpeedRunWidget`))
  (`/Engine/EditorBlueprintResources/StandardMacros.IsValid` _speedrunwidget
    (:`Is Valid`
      (`/Game/Blueprints/Widgets/Speedrun/WB_SpeedrunOverlay.UpdateStatCounter` _speedrunwidget))))

(fn `UserConstructionScript`
  (`parent.UserConstructionScript`))