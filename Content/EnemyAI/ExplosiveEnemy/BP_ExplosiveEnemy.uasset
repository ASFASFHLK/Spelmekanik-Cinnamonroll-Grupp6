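; Pooled explosive star enemy that charges up and deals radial damage on detonation.
; With Reactional music active, a quarter-note quantization callback steps the charge, growing the mesh and playing staged sounds before exploding on the third beat; otherwise a timed delay detonates it.
; Death stops AI, may fire a music stinger, then dissolves and returns it to the pool; spawning reverses the dissolve and restarts AI.
; Also handles being thrown, arced jumps and hit feedback.
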(event `self.ReceiveBeginPlay`
  (bind _asbp_rivet_game_instance (cast `/Game/Blueprints/Bp_RivetGameInstance` (`GameplayStatics.GetGameInstance`)))
  (set `self.As Bp Rivet Game Instance` _asbp_rivet_game_instance)
  (set `self.OriginalScale` (`SceneComponent.K2_GetComponentScale` (`self.Mesh`)))
  (`ReactionalPlaybackLibrary.MusicSystem_SubscribeToQuantizationEvent` "QuarterNote" (delegate `CountDownExplode`)))

(event `CountDownExplode`
  (bind _mesh (`self.Mesh`))
  (bind _returnvalue (`KismetMathLibrary.Conv_VectorToTransform` (`self.K2_GetActorLocation`)))
  (`FMODBlueprintStatics.SetGlobalParameterByName` "BPM" (`KismetMathLibrary.Conv_IntToDouble` (- (`ReactionalPlaybackLibrary.Playlist_GetTrack`) 1)))
  (if (`RivetGameInstance.ReactionalActivated` (`self.As Bp Rivet Game Instance`))
    (if (`self.Exploded`)
      (switch `int` (`self.ExplosionTriggerCount`)
        (:`0`
          (`FMODBlueprintStatics.PlayEventAtLocation` "/Game/FMOD/Events/SFX/Star/Star_ChargeUp_Stage1.Star_ChargeUp_Stage1" _returnvalue))
        (:`1`
          (`FMODBlueprintStatics.PlayEventAtLocation` "/Game/FMOD/Events/SFX/Star/Star_ChargeUp_Stage2.Star_ChargeUp_Stage2" _returnvalue))
        (:`2`
          _))
      (`SceneComponent.SetWorldScale3D` _mesh (+ (`SceneComponent.K2_GetComponentScale` _mesh) (0.1 0.1 0.1)))
      (bind _output_get (set `self.ExplosionTriggerCount` (+ (`self.ExplosionTriggerCount`) 1)))
      (if (>= _output_get 3)
        (set `self.ExplosionTriggerCount` 0)
        (`self.ActivateExplosion`)))))

(event `self.SetIsBeingThrown`
  (params (Value :type Boolean))
  ;[1 1 1] Enabled and disable collision when being thrown
  (`BlackboardComponent.SetValueAsBool` (`self.MyBlackBoard`) "BeingThrown" Value)
  (`PrimitiveComponent.SetCollisionEnabled` (`self.CapsuleComponent`) "NoCollision")
  (`KismetSystemLibrary.Delay` 0.5)
  (`PrimitiveComponent.SetCollisionEnabled` (`self.CapsuleComponent`) "QueryAndPhysics"))

(event `KillOnBeat`
  (if (>= (`ReactionalPlaybackLibrary.MusicSystem_GetTimeToBeat` 1.0) 0.5)
    (`ReactionalPlaybackLibrary.Theme_TriggerStinger_Quant` "KillOnBeat" "Instant")))

(event `self.Ragdoll`
  ;[1 1 1] Ragdoll
  (`PrimitiveComponent.SetCollisionEnabled` (`self.CapsuleComponent`) "NoCollision")
  (bind _braincomponent (`self.GetBrain`))
  (`BrainComponent.StopLogic` _braincomponent "")
  (`SceneComponent.SetHiddenInGame` (`self.NS_Chargeup`) true false)
  (`FMODAudioComponent.Stop` (`self.FMOD_ChargeUp`))
  (`FMODAudioComponent.Stop` (`self.FMOD_Walk`))
  (`FMODAudioComponent.Play` (`self.FMOD_Death`))
  (`SceneComponent.SetHiddenInGame` (`self.Vortex`) true false)
  (`self.KillOnBeat`)
  (bind (_direction _dissolve) (`Timeline|Timeline` :!via `PlayFromStart`)
    (:`Update`
      (`MeshComponent.SetScalarParameterValueOnMaterials` (`self.Mesh`) "Dissolve" _dissolve))
    (:`Finished`
      (`KismetSystemLibrary.Delay` 3.0)
      (`ObjectPooler.ReturnToPool` (subsystem `ObjectPooler`) self))))

(event `self.ReturnToPool`
  (bind _returnvalue (`self.GetMySquad`))
  ;[1 1 1] Return to pool and teleport to pool location
  (`self.ShutDownBehavior`)
  (`self.ReverseRagdoll`)
  (`self.ResetEnemy`)
  (`PrimitiveComponent.SetMaterial` (`self.Mesh`) 0 "/Game/VFX_MayBeDeleted/Dissolve/M_Dissolve_Star.M_Dissolve_Star")
  (if (`KismetSystemLibrary.IsValid` _returnvalue)
    (`self.K2_SetActorLocation` (`self.K2_GetActorLocation` _returnvalue) false true)
    (set `self.Exploded` false)))

(event `self.SpawnFromPool`
  ;[1 1 1] Spawn and activate logic
  (`SkeletalMeshComponent.PlayAnimation` (`self.Mesh`) "/Game/Animations/StarAnimations/StarRun_Anim.StarRun_Anim" true)
  (bind (_direction _dissolve) (`Timeline|Timeline_0` :!via `ReverseFromEnd`)
    (:`Update`
      (`MeshComponent.SetScalarParameterValueOnMaterials` (`self.Mesh`) "Dissolve" _dissolve))
    (:`Finished`
      (`SceneComponent.SetHiddenInGame` (`self.Vortex`) false false)
      (`SceneComponent.SetHiddenInGame` (`self.NS_Chargeup`) false false)
      (bind _braincomponent (`self.GetBrain`))
      (`BrainComponent.StartLogic` _braincomponent)
      (`FMODAudioComponent.Play` (`self.FMOD_Walk`)))))

(event `self.Explode`
  ;[1 1 1] Start explosion
  (`MovementComponent.StopMovementImmediately` (`self.CharacterMovement`))
  (`ActorComponent.Activate` (`self.NS_Chargeup`) false)
  (`SkeletalMeshComponent.PlayAnimation` (`self.Mesh`) "/Game/Animations/StarAnimations/StarAttack_Anim.StarAttack_Anim" false)
  (if (`self.GetIsAlive`)
    (set `self.Exploded` true)
    (if (`RivetGameInstance.ReactionalActivated` (`self.As Bp Rivet Game Instance`))
      (bind _asbp_default_game_mode (cast `/Game/BP_DefaultGameMode` (`GameplayStatics.GetGameMode`)))
      (if (`/Game/BP_DefaultGameMode.RoundActive` _asbp_default_game_mode)
        _)
      (else
        (`FMODAudioComponent.Play` (`self.FMOD_ChargeUp`))
        (`KismetSystemLibrary.Delay` 1.0)
        (`self.ActivateExplosion`)))))

(event `ActivateExplosion`
  ;[1 1 1] Activation of  explosion
  (if (`self.GetIsAlive`)
    (`self.BlowUp`)
    (`ActorComponent.Activate` (`self.EpxlodeStarTest`) false)
    (`FMODAudioComponent.Play` (`self.FMOD_Explode`)))
  (set `self.Exploded` false)
  (`SceneComponent.SetWorldScale3D` (`self.Mesh`) (`self.OriginalScale`)))

(event `self.TakeDamageVisual`
  ;[1 1 1] Visually take damage
  (`|PlayMontage` null "/Game/Animations/StarAnimations/StarTakeDamage_Anim_Montage.StarTakeDamage_Anim_Montage"
    (:`then`
      (`MeshComponent.SetOverlayMaterial` (`self.Mesh`) "/Game/Assets/Shaders/Material_Instances/Hit_Overlay_Instances/M_Hitoverlay_Star.M_Hitoverlay_Star")
      (`KismetSystemLibrary.Delay` 0.05)
      (`FMODBlueprintStatics.PlayEvent2D` "/Game/FMOD/Events/SFX/Player/Player_Gunshot_EnemyHit.Player_Gunshot_EnemyHit")
      (`KismetSystemLibrary.Delay` 0.05)
      (`MeshComponent.SetOverlayMaterial` (`self.Mesh`) "/Engine/Engine_MI_Shaders/Instances/M_Shader_SimpleTranslucent_Invis.M_Shader_SimpleTranslucent_Invis"))))

(event `/Game/EnemyAI/BPI_Enemy.JumpToDestination`
  (params (NewParam :type "Vector Structure"))
  ;[1 1 1] Jump function
  (`KismetSystemLibrary.Delay` 0.1)
  (bind _outlaunchvelocity (`GameplayStatics.SuggestProjectileVelocity_CustomArc` (`self.K2_GetActorLocation`) (`KismetMathLibrary.MakeVector` (.x NewParam) (.y NewParam) (+ (.z NewParam) 50.0))))
  (`self.LaunchCharacter` _outlaunchvelocity))

(event `self.ShutDownBehavior`
  ;[1 1 1] Stop enemy behavior and movement
  (bind _braincomponent (`self.GetBrain`))
  (`BrainComponent.StopLogic` _braincomponent "")
  (`MovementComponent.StopMovementImmediately` (`self.CharacterMovement`)))

(fn `BlowUp`
  (`GameplayStatics.ApplyRadialDamage` :`BaseDamage` (`self.GetDamage`) :`Origin` (`self.K2_GetActorLocation`) :`DamageRadius` (`self.GetExplosionRadius`) :`DamageTypeClass` "/Script/Engine.DamageType" :`DamageCauser` self :`InstigatedByController` (`self.GetController`) :`bDoFullDamage` true)
  (`self.HasDied`))

(fn `GetBrain`
  (returns (BrainComponent :type "BrainComponent Object Reference"))
  (return (`AIController.BrainComponent` (`AIBlueprintHelperLibrary.GetAIController` (`self.GetController`)))))

(fn `InitiateRagdoll`
  (`PrimitiveComponent.SetCollisionEnabled` (`self.CapsuleComponent`) "NoCollision")
  (`PrimitiveComponent.SetSimulatePhysics` (`self.Mesh`) true)
  (`PrimitiveComponent.SetCollisionEnabled` (`self.Mesh`) "QueryAndPhysics")
  (bind _braincomponent (`self.GetBrain`))
  (`BrainComponent.StopLogic` _braincomponent ""))

(fn `ReverseRagdoll`
  (bind _mesh (`self.Mesh`))
  (bind _mesh_2 (`self.Mesh`))
  (`PrimitiveComponent.SetCollisionEnabled` (`self.CapsuleComponent`) "QueryAndPhysics")
  (`PrimitiveComponent.SetSimulatePhysics` _mesh false)
  (`PrimitiveComponent.SetCollisionEnabled` _mesh "NoCollision")
  (`SceneComponent.K2_AttachToComponent` (`self.Mesh`) (`self.CapsuleComponent`) "None" "SnapToTarget" "KeepRelative" "KeepRelative" false)
  (`SceneComponent.K2_SetRelativeRotation` :`self` _mesh_2)
  (`SceneComponent.K2_SetRelativeLocation` _mesh_2 (0.0 0.0 -58.0) false true))

(fn `UserConstructionScript`)