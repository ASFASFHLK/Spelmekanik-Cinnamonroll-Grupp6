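; Main menu game mode that opens the menu widget with a visible cursor and starts the menu music.
; It creates a black-screen fade widget, which the screen effect event plays alongside a post-process material whose Pixels parameter is driven by a timeline.
; Two functions switch between the main and options menus, and between the General, Audio and Hotkeys pages, by adding and removing widgets from the viewport.
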(event `PlayScreenEffect`
  (params (PostVolume :type "PostProcessVolume Object Reference (by ref)") (EffectToPlay :type "MaterialInstanceDynamic Object Reference (by ref)"))
  (`/Game/Widgets/MainMenu/WBP_BlackScreen.PlayFadin` (`self.FadeOut`))
  (`MaterialInstanceDynamic.SetScalarParameterValue` EffectToPlay "Pixels" 5.0)
  (`PostProcessVolume.AddOrUpdateBlendable` PostVolume EffectToPlay 1.0)
  (bind (_direction _scalevalue) (`Timeline|Timeline` :`NewTime` 1.2 :!via `PlayFromStart`)
    (:`Update`
      (`MaterialInstanceDynamic.SetScalarParameterValue` EffectToPlay "Pixels" _scalevalue))))

(event `self.ReceiveBeginPlay`
  (bind _returnvalue (`|CreateWidget` "/Game/Widgets/MainMenu/WBP_BlackScreen.WBP_BlackScreen_C"))
  (bind _output_get (set `self.FadeOut` _returnvalue))
  (`UserWidget.AddToViewport` _output_get 0)
  (bind _returnvalue_2 (`|CreateWidget` "/Game/Widgets/MainMenu/WBP_MainMenu.WBP_MainMenu_C"))
  (`UserWidget.AddToViewport` _returnvalue_2 0)
  (set `PlayerController.bShowMouseCursor` true (`GameplayStatics.GetPlayerController` 0))
  (`Widget.SetVisibility` _returnvalue_2 "Visible")
  (`FMODBlueprintStatics.PlayEvent2D` "/Game/FMOD/Events/Music/MainMenu_ClinksAnthem.MainMenu_ClinksAnthem")
  (`ReactionalPlaybackLibrary.Playlist_SetVolume` 0.7)
  (`ReactionalPlaybackLibrary.Theme_SetVolume` 0.7))

(fn `SwapMainMenuAndOptions`
  (params (SwapToOptions :type Boolean))
  (bind _optionsmenu (`self.OptionsMenu`))
  (bind _mainmenu (`self.MainMenu`))
  (bind _generalmenu (`self.GeneralMenu`))
  (if SwapToOptions
    (`Widget.RemoveFromParent` _mainmenu)
    (`UserWidget.AddToViewport` _optionsmenu 0)
    (`UserWidget.AddToViewport` _generalmenu 0)
    (else
      (`Widget.RemoveFromParent` _optionsmenu)
      (`UserWidget.AddToViewport` _mainmenu 0)
      (`Widget.RemoveFromParent` _generalmenu)
      (`Widget.RemoveFromParent` (`self.HotkeyMenu`))
      (`Widget.RemoveFromParent` (`self.AudioMenu`)))))

(fn `SwapOptionsMenu`
  (params (MenuValue :type Integer))
  (switch `int` MenuValue
    (:`0`
      ;[1 1 1] Swap To General
      (`Widget.RemoveFromParent` (`self.AudioMenu`))
      (`Widget.RemoveFromParent` (`self.HotkeyMenu`))
      (`UserWidget.AddToViewport` (`self.GeneralMenu`) 0))
    (:`1`
      ;[1 1 1] Swap To Audio
      (`Widget.RemoveFromParent` (`self.GeneralMenu`))
      (`Widget.RemoveFromParent` (`self.HotkeyMenu`))
      (`UserWidget.AddToViewport` (`self.AudioMenu`) 0))
    (:`2`
      ;[1 1 1] Swap To Hotkeys
      (`Widget.RemoveFromParent` (`self.GeneralMenu`))
      (`Widget.RemoveFromParent` (`self.AudioMenu`))
      (`UserWidget.AddToViewport` (`self.HotkeyMenu`) 0))))

(fn `UserConstructionScript`)